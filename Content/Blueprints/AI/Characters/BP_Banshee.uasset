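; BP_Banshee is an AI enemy character that attacks with an area-of-effect spell.
; On BeginPlay it loads its attack row from DT_EnemyAOE and scales the damage range by DamageMultiplier.
; CastSpell spawns a BP_BansheeAOE at CastingPoint with that radius, knockback and a random damage roll, then triggers its attack.
; Cast begin and end events toggle the attack flags, and GetAIData exposes AI settings, state and target.
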(event EventBeginPlay
  (|CallParentFunction)
  (CallFunction|SetAOEData "/Game/Blueprints/Data/Characters/Enemies/DT_EnemyAOE.DT_EnemyAOE" (Variables|Default|GetAOEAttackRowName)))

(event EventOnBindtoGameMode
  (|CallParentFunction))

(event EventSpellCastEnded
  (Variables|Default|SetCanAttack true)
  (Variables|Default|SetIsAttacking false))

(event EventSpellCastBegun
  (Variables|Default|SetCanAttack false)
  (Variables|Default|SetIsAttacking true))

(event EventTick
  (params (DeltaSeconds :type Float%20%28single-precision%29))
  (|CallParentFunction DeltaSeconds))

(event EventCastSpell
  (bind _aoeattackdata (Variables|AIData|GetAOEAttackData))
  (bind _returnvalue (Game|SpawnActorfromClass "/Game/Blueprints/Weapon/Enemy/BP_BansheeAOE.BP_BansheeAOE_C" (Math|Transform|MakeTransform (Transformation|GetWorldLocation (Variables|Default|GetCastingPoint)) "0, 0, 0" "1,1,1") "Undefined" 0 (.range _aoeattackdata) (Math|Random|RandomFloatinRange (.mindamage _aoeattackdata) (.maxdamage _aoeattackdata)) (.knockback _aoeattackdata) self))
  (Default|OnAttack _returnvalue))

(fn ConstructionScript
  (|CallParentFunction))

(fn GetAIData
  (bind _aidata (Variables|Default|GetAIData))
  (return (.attackrange _aidata) (.wanderrange _aidata) (.closecombatrange _aidata) (.wanderwaittime _aidata) (.meleeattackrate _aidata) (.rangedattackrate _aidata) (.defaultaistate _aidata) (Variables|Default|GetcurrentState) (Variables|Default|GetcurrentTarget)))

(fn InitChase
  (|CallParentFunction))

(fn SetAOEData
  (params (DataTable :type Data%20Table%20Object%20Reference) (RowName :type Name))
  (bind _damage_multiplier (Variables|Default|GetDamage%20Multiplier))
  (bind _returnvalue (Utilities|GetDataTableRow DataTable RowName)
    (:then
      (bind _structout (Utilities|Struct|SetmembersinS_AOEAttackData _returnvalue (* _damage_multiplier (.MaxDamage (Utilities|Struct|BreakS_AOEAttackData _returnvalue))) (* _damage_multiplier (.MinDamage (Utilities|Struct|BreakS_AOEAttackData _returnvalue)))))
      (Variables|AIData|SetAOEAttackData _structout))))
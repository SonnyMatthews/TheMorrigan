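; Base enemy character that loads stats and loot from data tables, with a health widget and optional elite shield or status-effect component.
; A state enum sets walk speed and fires state triggers; the vision sphere starts a chase on the player, and Tick turns attackers toward their target.
; Damage not blocked by a shield spawns damage numbers, then either staggers with knockback, flash and brief invulnerability, or kills and rolls loot.
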(event OnComponentBeginOverlap(VisionArea)
  (params (OverlappedComponent :type Primitive%20Component%20Object%20Reference) (OtherActor :type Actor%20Object%20Reference) (OtherComp :type Primitive%20Component%20Object%20Reference) (OtherBodyIndex :type Integer) (bFromSweep :type Boolean) (SweepResult :type Hit%20Result%20Structure%20%28by%20ref%29))
  (Utilities|IsValid (Variables|AIData|GetcurrentTarget)
    (:Is%20Not%20Valid
      (if (Actor|ActorHasTag OtherActor "Player")
        (CallFunction|SetTarget OtherActor)
        (CallFunction|SetNewState "NewEnumerator3")
        (Default|CallOnNewStateTrigger (Variables|AIData|GetcurrentState))))))

(event Custom|OnBindToGameMode
  (bind _gamemode (Class|IMorriganGameMode|GetGameModeRef(Message) (Game|GetGameMode)))
  (EventDispatchers|BindEventtoOnNewState _gamemode (delegate Custom|OnNewGameState)))

(event Custom|OnNewGameState
  (params (NewState :type E_GameStates%20Enum :default "NewEnumerator0"))
  (switch Utilities|FlowControl|Switch|SwitchonE_GameStates NewState
    (:NewEnumerator3
      _)
    (:NewEnumerator9
      _))
  (Default|CallOnNewStateTrigger "NewEnumerator1"))

(event EventBeginPlay
  (bind _output_get (Variables|Default|SetLootTable "/Game/Blueprints/Data/Loot/DT_EnemyLootTable.DT_EnemyLootTable"))
  (CallFunction|SetLootTable _output_get (Variables|Default|GetLootTableRowName))
  (CallFunction|SetAIData (Variables|AIData|GetDT_AIData) (Variables|Default|GetDataRowName))
  (bind _asaic_base_enemy (Utilities|Casting|CastToAIC_BaseEnemy (Pawn|GetController)))
  (bind _output_get_2 (Variables|Components|SetaiController _asaic_base_enemy))
  (Default|Init _output_get_2)
  (bind _returnvalue (UserInterface|CreateWidget "/Game/Blueprints/UI/Widget_EnemyHealth.Widget_EnemyHealth_C"))
  (bind _output_get_3 (Variables|Default|SetHealthWidget _returnvalue))
  (UserInterface|SetWidget (Variables|Default|GetHealth) _output_get_3)
  (CallFunction|EvaluateCurrentState)
  (Default|CallOnNewStateTrigger (Variables|AIData|GetcurrentState))
  (CallFunction|OnBindtoGameMode)
  (CallFunction|SetUpElite))

(event EventUpdateState
  (params (NewState :type E_BaseEnemyStates%20Enum :default "NewEnumerator0"))
  (CallFunction|SetNewState NewState))

(event EventFinishHurt
  (Utilities|Time|PauseTimerbyHandle (Variables|Default|GetFlashTimerHandle))
  (CallFunction|FlashOff)
  (Variables|Default|SetisHurt false))

(event EventTick
  (params (DeltaSeconds :type Float%20%28single-precision%29))
  (Utilities|SwitchCurrentState
    (:Attack
      (if (not (Variables|States|GetIsAttacking))
        (Utilities|IsValid (Variables|AIData|GetcurrentTarget)
          (:Is%20Valid
            (Transformation|SetActorRotation (Math|Rotator|MakeRotator 0.0 0.0 (.yaw (Math|Interpolation|RInterpTo (Transformation|GetActorRotation) (Math|Rotator|FindLookatRotation (Transformation|GetActorLocation) (Transformation|GetActorLocation (Variables|AIData|GetcurrentTarget))) DeltaSeconds 2.5))))))))))

(event EventMeleeBegun
  (Variables|States|SetCanAttack false)
  (Variables|States|SetIsAttacking true))

(event EventMeleeEnd
  (Variables|States|SetIsAttacking false)
  (Variables|States|SetCanAttack true))

(event EventTargetDestroyed
  (CallFunction|SetNewState (.defaultaistate (Variables|AIData|GetAIData))))

(event EventDamage
  (params (Damage :type Float%20%28single-precision%29) (KnockBack :type Float%20%28single-precision%29) (InterfacingActor :type Actor%20Object%20Reference) (ActorLocation :type Vector :default "0, 0, 0"))
  (Utilities|IsValid (Variables|Default|GetShieldComponent)
    (:Is%20Valid
      (bind _isalive (Default|IsShieldAlive (Variables|Default|GetShieldComponent)))
      (if (not _isalive)
        (if (not (Variables|Default|GetisHurt)) :!label _label
          (bind _isdead_ (CallFunction|DeductHealth Damage))
          (if _isdead_
            (CallFunction|CreateDamageVFX Damage "(R=1.000000,G=1.000000,B=1.000000,A=1.000000)" (Math|Vector|GetUnitDirection(Vector) ActorLocation (Transformation|GetActorLocation)))
            (CallFunction|GenerateLootDrops)
            (CallFunction|Death)
            (else
              (CallFunction|UpdateHealth)
              (Class|IWeapon|IDeactivateWeaponHitbox(Message) (Variables|/Script/Engine.ChildActorComponent|GetChildActor (Variables|Default|GetWeapon)))
              (CallFunction|OnHurt)
              (CallFunction|SetNewState "NewEnumerator4")
              (Default|CallOnNewStateTrigger "NewEnumerator4")
              (CallFunction|AddImpulseinDirection ActorLocation KnockBack)
              (CallFunction|CreateDamageVFX Damage "(R=1.000000,G=1.000000,B=1.000000,A=1.000000)" (Math|Vector|GetUnitDirection(Vector) ActorLocation (Transformation|GetActorLocation)))
              (Animation|Montage|MontageStop (Components|SkeletalMesh|GetAnimInstance (Variables|Character|GetMesh)) 0.1 0)
              (Animation|Montage|PlayMontage (Variables|Character|GetMesh) "/Game/Animation/Temporary/AM_TempStagger.AM_TempStagger"
                (:OnCompleted
                  (CallFunction|SetNewState "NewEnumerator2")
                  (Default|CallOnNewStateTrigger "NewEnumerator2")
                  (Development|PrintString "COMPLETE?"))))))))
    (:Is%20Not%20Valid
      (goto _label))))

(event EventOnHurt
  (Variables|Default|SetisHurt true)
  (Utilities|Time|SetTimerbyEvent (delegate EventFinishHurt) (Variables|Default|GethurtTime))
  (CallFunction|Flashon))

(fn ConstructionScript
  (|CallParentFunction))

(fn EvaluateCurrentState
  (Utilities|SwitchCurrentState
    (:Idle
      (CallFunction|InitIdle))
    (:Wander
      (CallFunction|InitWander))
    (:Attack
      (CallFunction|InitAttack))
    (:Chase
      (CallFunction|InitChase))))

(fn SetNewState
  (params (currentState :type E_BaseEnemyStates%20Enum :default "NewEnumerator0"))
  (Variables|AIData|SetcurrentState currentState)
  (CallFunction|EvaluateCurrentState))

(fn InitChase
  (Variables|/Script/Engine.CharacterMovementComponent|SetMaxWalkSpeed (Variables|Character|GetCharacterMovement) (.chasespeed (Variables|AIData|GetAIData))))

(fn InitAttack
  (Variables|/Script/Engine.CharacterMovementComponent|SetMaxWalkSpeed (Variables|Character|GetCharacterMovement) 0.0))

(fn InitWander
  (Variables|/Script/Engine.CharacterMovementComponent|SetMaxWalkSpeed (Variables|Character|GetCharacterMovement) (.wanderspeed (Variables|AIData|GetAIData))))

(fn InitIdle)

(fn SetAIData
  (params (DataTable :type Data%20Table%20Object%20Reference) (RowName :type Name))
  (bind _returnvalue (Utilities|GetDataTableRow DataTable RowName)
    (:then
      (bind _output_get (Variables|AIData|SetAIData _returnvalue))
      (bind _structout (Utilities|Struct|SetmembersinS_AIData _output_get))
      (Components|Sphere|SetSphereRadius (Variables|Default|GetVisionArea) (.detectionrange _structout) false)
      (Variables|Default|SetCurrentHealth (* (.maxhealth _structout) (Variables|Stats|GetHealth%20Multiplier)))
      (Class|IWeapon|SetDamageMultiplier(Message) (Variables|/Script/Engine.ChildActorComponent|GetChildActor (Variables|Default|GetWeapon)) (Variables|Stats|GetDamage%20Multiplier))
      (bind _output_get_2 (Variables|Default|SetMeleeAttackAnimationData (Utilities|Struct|BreakS_AIData (Variables|AIData|GetAIData))))
      (Utilities|Map|Keys (Utilities|Struct|BreakS_AttackAnimationData _output_get_2)))))

(fn SetTarget
  (params (NewTarget :type Actor%20Object%20Reference))
  (Variables|AIData|SetcurrentTarget NewTarget))

(fn DoAttackAnim
  (Variables|/Script/Engine.CharacterMovementComponent|SetMaxWalkSpeed (Variables|Character|GetCharacterMovement) 0.0)
  (Animation|PlayAnimMontage "/Game/CloseCombat/AM_EnemyAttack.AM_EnemyAttack" 1.0 "None"))

(fn ResetAttackTimers
  (Utilities|Time|PauseTimerbyHandle (Variables|Timers|GetMeleeAttackTimer)))

(fn ResetAttackMeleeCooldown
  (if (not (Variables|States|GetCanAttack))
    (Variables|States|SetCanAttack true)))

(fn Death
  (|CallParentFunction)
  (Actor|DestroyActor))

(fn UpdateHealth
  (|CallParentFunction)
  (Default|UpdateHealth (Variables|Default|GetHealthWidget) (/ (Variables|Default|GetCurrentHealth) (.MaxHealth (Utilities|Struct|BreakS_AIData (Variables|AIData|GetAIData))))))

(fn InAttackRange
  (Utilities|IsValid (Variables|AIData|GetcurrentTarget)
    (:Is%20Valid
      (return (<= (Math|Vector|Distance(Vector) (Transformation|GetActorLocation) (Transformation|GetActorLocation (Variables|AIData|GetcurrentTarget))) (.attackrange (Variables|AIData|GetAIData)))))
    (:Is%20Not%20Valid
      (return false))))

(fn InCloseAttackRange
  (Utilities|IsValid (Variables|AIData|GetcurrentTarget)
    (:Is%20Valid
      (return (<= (Math|Vector|Distance(Vector) (Transformation|GetActorLocation) (Transformation|GetActorLocation (Variables|AIData|GetcurrentTarget))) (.closecombatrange (Variables|AIData|GetAIData)))))
    (:Is%20Not%20Valid
      (return false))))

(fn IGetMesh
  (return (Variables|Character|GetMesh)))

(fn CreateDamageVFX
  (params (damage :type Float%20%28single-precision%29) (textColour :type Linear%20Color%20Structure) (driftDir :type Vector))
  (bind _returnvalue (Transformation|GetActorLocation))
  (LocalVariables|SetpercentageDIF (/ damage (.maxhealth (Variables|AIData|GetAIData))))
  (bind _output_get (LocalVariables|SetColor textColour))
  (LocalVariables|SetColor (Utilities|Struct|MakeLinearColor (.r _output_get) (- 1.0 (LocalVariables|GetpercentageDIF)) (- 1.0 (LocalVariables|GetpercentageDIF)) (.a _output_get)))
  (bind _randpoint (CallFunction|GetRandPointinSphere (Math|Vector|MakeVector (.x _returnvalue) (.y _returnvalue) (+ (.z _returnvalue) 1e+02)) 1e+01))
  (Game|SpawnActorfromClass "/Game/Blueprints/VFX/BP_DamageNumber.BP_DamageNumber_C" (Math|Transform|MakeTransform _randpoint "0, 0, 0" "1,1,1") "Undefined" 0 damage (LocalVariables|GetColor) driftDir (.maxhealth (Variables|AIData|GetAIData)) 0))

(fn SetLootTable
  (params (DataTable :type Data%20Table%20Object%20Reference) (RowName :type Name))
  (bind _returnvalue (Utilities|GetDataTableRow DataTable RowName)
    (:then
      (Variables|AIData|SetLootData _returnvalue))))

(fn GenerateLootDrops
  (bind _lootdata (Variables|AIData|GetLootData))
  (bind _lootdata_2 (Variables|AIData|GetLootData))
  (bind _returnvalue (Utilities|Array|LastIndex (.drops _lootdata_2)))
  (bind _returnvalue_2 (Math|Random|RandomIntegerinRange 0 _returnvalue))
  (bind _output (Utilities|Array|Get(acopy) (.drops _lootdata_2) _returnvalue_2))
  (for _index (range 0 (Math|Random|RandomIntegerinRange (.mindrops _lootdata) (.maxdrops _lootdata)))
    (if (<= (Math|Random|RandomFloat) (.dropchance _output))
      (CallFunction|SpawnLootDrop (.dropactor _output)))))

(fn SpawnLootDrop
  (params (lootClass :type Actor%20Class%20Reference))
  (Game|SpawnActorfromClass lootClass (Math|Transform|MakeTransform (Transformation|GetWorldLocation (Variables|Character|GetMesh)) "0, 0, 0" "1,1,1") "Undefined" 0 0))

(fn InitStagger
  (Variables|/Script/Engine.CharacterMovementComponent|SetMaxWalkSpeed (Variables|Character|GetCharacterMovement) 0.0))

(fn SetUpElite
  (if (Variables|States|GetisElite)
    (switch Utilities|FlowControl|Switch|SwitchonE_EliteAttributeType (Variables|States|GetEliteAttributeType)
      (:NewEnumerator0
        (bind _returnvalue (AddComponent|AddBPCShieldAttribute))
        (bind _output_get (Variables|Default|SetShieldComponent _returnvalue))
        (Default|Init _output_get))
      (:NewEnumerator1
        (bind _returnvalue_2 (AddComponent|AddBPCStatusEffectAttribute))
        (bind _output_get_2 (Variables|Default|SetStatusEffectComponent _returnvalue_2))
        (Default|Init _output_get_2 (Variables|States|GetStatusEffectType))))))

(fn GetHUD
  (return 0))

(fn GetPlayerController
  (return 0))

(fn GetAIData
  (bind _aidata (Variables|AIData|GetAIData))
  (bind (_attackrange _wanderrange _wanderspeed _wanderwaittime _defaultaistate _closecombatrange _detectionrange _meleeattackrate _rangedattackrate) (Utilities|Struct|BreakS_AIData _aidata))
  (return _attackrange _wanderrange _closecombatrange _wanderwaittime _meleeattackrate _rangedattackrate _defaultaistate (Variables|AIData|GetcurrentState) (Variables|AIData|GetcurrentTarget)))

(fn GetEliteAttributeType
  (return "NewEnumerator0"))

(fn GetIsAttacking
  (return (Variables|States|GetIsAttacking)))

(fn GetIsElite
  (return false))

(fn GetMontages
  (return 0 0))

(fn GetWeapon
  (bind _asbp_base_weapon (Utilities|Casting|CastToBP_BaseWeapon (Variables|/Script/Engine.ChildActorComponent|GetChildActor (Variables|Default|GetWeapon))))
  (return _asbp_base_weapon))

(fn IAddHealth
  (params (HealthToAdd :type Float%20%28single-precision%29))
  (return false))

(fn IGetMeleeAnimationData
  (return ""))
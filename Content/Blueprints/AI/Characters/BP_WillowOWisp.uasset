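; BP_WillowOWisp is a floating wisp AI character that drifts in random directions through a ProjectileMovement component.
; Init picks Chase or Wander from Target validity, though only Idle and Wander have behavior in EvaluateState.
; Wandering uses randomized timers to choose Z-clamped directions, blended in by a slowed timeline.
; Tick sets velocity to the sum of wander and evade forces, with evade never assigned here.
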(event Custom|OnStopWanderTransition
  (bind _wandertimeline (Timeline|WanderTransitionTime Stop)
    (:Update
      (Variables|Default|SetCurrentwanderForce (Math|Vector|Lerp(Vector) (Variables|Default|GetCurrentwanderForce) (Variables|Default|GettargetWanderForce) _wandertimeline)))
    (:Finished
      (bind _returnvalue (Utilities|Time|SetTimerbyFunctionName 0 "ChangeWanderDirection" (Math|Random|RandomFloatinRange (Variables|Default|GetmaxTimeBtwnWanderDir) (Variables|Default|GetminTimeBtwnWanderDir))))
      (Variables|Default|SetWanderChangeHandle _returnvalue))))

(event Custom|OnNewWanderForce
  (bind _wandertimeline (Timeline|WanderTransitionTime PlayFromStart)
    (:Update
      (Variables|Default|SetCurrentwanderForce (Math|Vector|Lerp(Vector) (Variables|Default|GetCurrentwanderForce) (Variables|Default|GettargetWanderForce) _wandertimeline)))
    (:Finished
      (bind _returnvalue (Utilities|Time|SetTimerbyFunctionName 0 "ChangeWanderDirection" (Math|Random|RandomFloatinRange (Variables|Default|GetmaxTimeBtwnWanderDir) (Variables|Default|GetminTimeBtwnWanderDir))))
      (Variables|Default|SetWanderChangeHandle _returnvalue))))

(event EventBeginPlay
  (CallFunction|Init))

(event EventTick
  (params (DeltaSeconds :type Float%20%28single-precision%29))
  (bind _output_get (Variables|Default|SetnetVelocity (+ (Variables|Default|GetevadeForce) (Variables|Default|GetCurrentwanderForce))))
  (Variables|/Script/Engine.MovementComponent|SetVelocity (Variables|Default|GetProjectileMovement) _output_get))

(fn ConstructionScript)

(fn GetRandomDirection
  (bind _randpoint (CallFunction|GetRandomPointinSphere (Transformation|GetActorLocation) (Variables|Default|GetWanderRange)))
  (return (- _randpoint (Transformation|GetActorLocation))))

(fn GetRandomPointinSphere
  (params (centre :type Vector) (radius :type Float%20%28single-precision%29))
  (return (+ centre (* (Math|Random|RandomUnitVector) (Math|Random|RandomFloatinRange 0.0 radius)))))

(fn Init
  (Components|Timeline|SetPlayRate (Variables|Default|GetWanderTransitionTime) 0.25)
  (Utilities|IsValid (Variables|Default|Gettarget)
    (:Is%20Valid
      (Variables|Default|SetcurrentState "NewEnumerator3"))
    (:Is%20Not%20Valid
      (Variables|Default|SetcurrentState "NewEnumerator1")))
  (CallFunction|EvaluateState))

(fn EvaluateState
  (Utilities|SwitchState
    (:Idle
      (Variables|/Script/Engine.ProjectileMovementComponent|SetMaxSpeed (Variables|Default|GetProjectileMovement) 0.0))
    (:Wander
      (CallFunction|InitWander))))

(fn InitWander
  (Variables|/Script/Engine.ProjectileMovementComponent|SetMaxSpeed (Variables|Default|GetProjectileMovement) (Variables|Default|GetmaxWanderSpeed))
  (bind _randdir (CallFunction|GetRandomDirection))
  (Variables|Default|SetCurrentwanderForce (Math|Vector|MakeVector (.x (* _randdir (Variables|Default|GetmaxWanderSpeed))) (.y (* _randdir (Variables|Default|GetmaxWanderSpeed))) (Math|Float|Clamp(Float) (.z (* _randdir (Variables|Default|GetmaxWanderSpeed))) (Variables|Default|GetMinZ) (Variables|Default|GetMaxZ))))
  (bind _returnvalue (Utilities|Time|SetTimerbyFunctionName 0 "ChangeWanderDirection" (Math|Random|RandomFloatinRange (Variables|Default|GetmaxTimeBtwnWanderDir) (Variables|Default|GetminTimeBtwnWanderDir))))
  (Variables|Default|SetWanderChangeHandle _returnvalue))

(fn ChangeWanderDirection
  (if (Utilities|Enum|Equal(Enum) (Variables|Default|GetcurrentState) "NewEnumerator1")
    (bind _randdir (CallFunction|GetRandomDirection))
    (Variables|Default|SettargetWanderForce (Math|Vector|MakeVector (.x (* _randdir (Variables|Default|GetmaxWanderSpeed))) (.y (* _randdir (Variables|Default|GetmaxWanderSpeed))) (Math|Float|Clamp(Float) (.z (* _randdir (Variables|Default|GetmaxWanderSpeed))) (Variables|Default|GetMinZ) (Variables|Default|GetMaxZ))))
    (CallFunction|OnNewWanderForce)))
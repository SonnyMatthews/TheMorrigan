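; Witch AI character, a child of a parent AI class, that channels and fires projectile spells, with flags tracking melee, channel and cast phases.
; Data table rows supply AI stats and projectile stats, with damage scaled by a multiplier.
; BeginAttackSpell grows a child-actor VFX at CastingPoint by timeline, then spawns the projectile, while CastSpell spawns one homing on the current target.
; An Idle/Wander/Attack/Chase switch dispatches state initialisation.
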(event Custom|BeginAttackSpell
  (bind _castingpoint (Variables|Default|GetCastingPoint))
  (bind _castingpoint_2 (Variables|Default|GetCastingPoint))
  (bind _castingpoint_3 (Variables|Default|GetCastingPoint))
  (bind _spelldata (Variables|AIData|GetSpellData))
  ;[1 1 1] If already channelling spell don't  start again
  (if (not (Variables|AttackSettings|GetIsChannelling))
    (Variables|AttackSettings|SetIsChannelling true)
    ;[1 1 1] Initialise casting anim
    (Transformation|SetWorldScale3D _castingpoint "0, 0, 0")
    (ChildActorComponent|SetChildActorClass _castingpoint (Variables|Default|GetSpellVFX))
    (bind _channelcurve (Timeline|ChannelTimeLine PlayFromStart)
      (:Update
        (Transformation|SetWorldScale3D _castingpoint_3 (Math|Vector|Lerp(Vector) (Transformation|GetWorldScale _castingpoint_3) (Variables|Default|GetMaxSpellVFXScale) _channelcurve)))
      (:Finished
        (Utilities|FlowControl|Delay 0.5)
        (ChildActorComponent|SetChildActorClass (Variables|Default|GetCastingPoint) 0)
        (Game|SpawnActorfromClass (Variables|Default|GetSpell) (Math|Transform|MakeTransform (Transformation|GetWorldLocation _castingpoint_2) (Math|Rotator|MakeRotfromX (Math|Vector|GetForwardVector _castingpoint_2)) "1,1,1") "Undefined" 0 0 (.projectiledamage _spelldata) (.projectilestartspeed _spelldata) (.projectilemaxspeed _spelldata) (.gravity _spelldata) (.lifespan _spelldata) (.maxenemycanhit _spelldata) (Transformation|GetWorldScale _castingpoint_2) 0)
        (Variables|AttackSettings|SetIsChannelling false)))))

(event EventBeginPlay
  ;[1 1 1] Begin
  (|CallParentFunction)
  (CallFunction|SetSpellData (Variables|AIData|GetSpellDT) (Variables|AIData|GetSpellName))
  (ChildActorComponent|SetChildActorClass (Variables|Default|GetCastingPoint) 0)
  (Variables|Default|SetMaxSpellVFXScale (Transformation|GetWorldScale (Variables|Default|GetCastingPoint))))

(event EventOnBindtoGameMode
  (|CallParentFunction))

(event EventTargetDestroyed
  (CallFunction|SetNewState (.defaultaistate (Variables|Default|GetAIData))))

(event EventUpdateState
  (params (NewState :type E_BaseEnemyStates%20Enum :default "NewEnumerator0"))
  (CallFunction|SetNewState NewState))

(event EventSpellCastEnded
  (Variables|Default|SetCanAttack true)
  (Variables|Default|SetIsAttacking false))

(event EventSpellCastBegun
  (Variables|Default|SetCanAttack false)
  (Variables|Default|SetIsAttacking true))

(event EventTick
  (params (DeltaSeconds :type Float%20%28single-precision%29))
  ;[1 1 1] Event Tick
  (|CallParentFunction DeltaSeconds))

(event EventMeleeBegun
  (Variables|AttackSettings|SetIsChannelling false)
  (Variables|Default|SetIsAttacking false)
  (Variables|Default|SetCanAttack true))

(event EventMeleeEnd
  (Variables|Default|SetCanAttack false)
  (Variables|Default|SetIsAttacking true))

(event EventCastSpell
  (bind _spelldata (Variables|AIData|GetSpellData))
  (bind _castingpoint (Variables|Default|GetCastingPoint))
  (Game|SpawnActorfromClass (Variables|Default|GetSpell) (Math|Transform|MakeTransform (Transformation|GetWorldLocation _castingpoint) (Math|Rotator|MakeRotfromX (Math|Vector|GetForwardVector _castingpoint)) "1,1,1") "Undefined" 0 (Variables|/Script/Engine.Actor|GetRootComponent (Variables|Default|GetcurrentTarget)) (.projectiledamage _spelldata) (.projectilestartspeed _spelldata) (.projectilemaxspeed _spelldata) (.gravity _spelldata) (.lifespan _spelldata) (.maxenemycanhit _spelldata) (Transformation|GetWorldScale _castingpoint) 0)
  (Variables|AttackSettings|SetIsChannelling false))

(event EventChannelBegin
  (Variables|AttackSettings|SetIsChannelling true)
  (Variables|Default|SetIsAttacking false))

(event EventChannelFinished
  (Variables|AttackSettings|SetIsChannelling false)
  (Variables|Default|SetIsAttacking false))

(fn ConstructionScript
  (|CallParentFunction))

(fn InitAttack
  (|CallParentFunction))

(fn EvaluateCurrentState
  (Utilities|SwtichState
    (:Idle
      (CallFunction|InitIdle))
    (:Wander
      (CallFunction|InitWander))
    (:Attack
      (CallFunction|InitAttack))
    (:Chase
      (CallFunction|InitChase)))
  (Variables|AttackSettings|SetIsChannelling false))

(fn SetSpellData
  (params (DataTable :type Data%20Table%20Object%20Reference) (RowName :type Name))
  (bind _returnvalue (Utilities|GetDataTableRow DataTable RowName)
    (:then
      (bind _structout (Utilities|Struct|SetmembersinS_ProjectileStats _returnvalue (* (.ProjectileDamage (Utilities|Struct|BreakS_ProjectileStats _returnvalue)) (Variables|Default|GetDamage%20Multiplier))))
      (Variables|AIData|SetSpellData _structout))))

(fn SetAIData
  (params (DataTable :type Data%20Table%20Object%20Reference) (RowName :type Name :default "None"))
  (bind _returnvalue (Utilities|GetDataTableRow DataTable RowName)
    (:then
      (bind _output_get (Variables|Default|SetAIData _returnvalue))
      (bind _structout (Utilities|Struct|SetmembersinS_AIData _output_get))
      (Components|Sphere|SetSphereRadius (Variables|Default|GetVisionArea) (.detectionrange _structout) false)
      (Variables|Default|SetCurrentHealth (.maxhealth _structout))
      (Variables|Default|SetMeleeAttackAnimationData (.meleeattack_stats _structout))
      (if true
        _))))
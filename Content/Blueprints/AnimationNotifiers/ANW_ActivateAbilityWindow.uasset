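; Anim notify state that marks an ability window in an animation, activating and deactivating a configured ability on the mesh's owner.
; On begin, it messages the owner with the ability and the active montage's remaining play time as the time until cooldown activates, also printing that time.
; On end, it sends the owner the matching deactivate interface message.
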(fn ReceivedNotifyBegin
  (params (MeshComp :type Skeletal%20Mesh%20Component%20Object%20Reference) (Animation :type Anim%20Sequence%20Base%20Object%20Reference) (TotalDuration :type Float%20%28single-precision%29))
  (bind _returnvalue (Components|SkeletalMesh|GetAnimInstance MeshComp))
  (bind _returnvalue_2 (Animation|Montage|GetCurrentActiveMontage _returnvalue))
  (bind _returnvalue_3 (Animation|GetPlayLength _returnvalue_2))
  (Development|PrintString 0 (Utilities|String|ToString(Float) (- _returnvalue_3 (Animation|Montage|MontageGetPosition _returnvalue _returnvalue_2))))
  (Class|ICharacter|IActivateAbility(Message) (Components|GetOwner MeshComp) (Variables|Default|GetAbilityToActivate) (- _returnvalue_3 (Animation|Montage|MontageGetPosition _returnvalue _returnvalue_2)))
  (return false))

(fn ReceivedNotifyEnd
  (params (MeshComp :type Skeletal%20Mesh%20Component%20Object%20Reference) (Animation :type Anim%20Sequence%20Base%20Object%20Reference))
  (Class|ICharacter|IDeactivateAbility(Message) (Components|GetOwner MeshComp) (Variables|Default|GetAbilityToActivate))
  (return false))
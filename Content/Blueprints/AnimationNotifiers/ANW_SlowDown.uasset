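; ANW_SlowDown is an anim notify state that changes montage playback speed over a marked window of an animation.
; On begin, it sets the play rate of the mesh anim instance's current active montage to SlowDown.
; On end, it sets whichever montage is then active to SpeedOut, rather than restoring a saved rate or using the notifying animation.
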(fn ReceivedNotifyBegin
  (params (MeshComp :type Skeletal%20Mesh%20Component%20Object%20Reference) (Animation :type Anim%20Sequence%20Base%20Object%20Reference) (TotalDuration :type Float%20%28single-precision%29))
  (bind _returnvalue (Components|SkeletalMesh|GetAnimInstance MeshComp))
  (Animation|Montage|MontageSetPlayRate _returnvalue (Animation|Montage|GetCurrentActiveMontage _returnvalue) (Variables|Default|GetSlowDown))
  (return false))

(fn ReceivedNotifyEnd
  (params (MeshComp :type Skeletal%20Mesh%20Component%20Object%20Reference) (Animation :type Anim%20Sequence%20Base%20Object%20Reference))
  (bind _returnvalue (Components|SkeletalMesh|GetAnimInstance MeshComp))
  (Animation|Montage|MontageSetPlayRate _returnvalue (Animation|Montage|GetCurrentActiveMontage _returnvalue) (Variables|Default|GetSpeedOut))
  (return false))
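; Anim notify that tells the mesh's owning actor to activate a chosen ability at a point in a montage.
; It sends the ability through an interface message along with the montage's remaining play time, used as the delay until cooldown starts.
; An unconnected leftover branch would spawn the ability actor and trigger its cooldown directly.
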(fn ReceivedNotify
  (params (MeshComp :type Skeletal%20Mesh%20Component%20Object%20Reference) (Animation :type Anim%20Sequence%20Base%20Object%20Reference))
  (bind _returnvalue (Components|SkeletalMesh|GetAnimInstance MeshComp))
  (bind _returnvalue_2 (Animation|Montage|GetCurrentActiveMontage _returnvalue))
  (bind _returnvalue_3 (Animation|GetPlayLength _returnvalue_2))
  (Class|ICharacter|IActivateAbility(Message) (Components|GetOwner MeshComp) (Variables|Default|GetAbilityToActivate) (- _returnvalue_3 (Animation|Montage|MontageGetPosition _returnvalue _returnvalue_2)))
  (return false))
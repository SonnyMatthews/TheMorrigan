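; Anim notify that turns on the equipped weapon's hitbox during a melee attack montage.
; It gets the weapon and melee attack data from the mesh owner through interface messages.
; Damage and knockback come from nested map lookups keyed by the active montage, then its current section as the combo name, and are passed to the weapon's hitbox activation message.
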(fn ReceivedNotify
  (params (MeshComp :type Skeletal%20Mesh%20Component%20Object%20Reference) (Animation :type Anim%20Sequence%20Base%20Object%20Reference))
  (bind _returnvalue (Components|GetOwner MeshComp))
  (bind _returnvalue_2 (Components|SkeletalMesh|GetAnimInstance MeshComp))
  (bind _weaponequipped (Class|IPawn|IGetWeaponEquipped(Message) _returnvalue))
  (LocalVariables|SetTempWeapon _weaponequipped)
  (bind _meleeattackanimationdata (Class|IPawn|IGetMeleeAttackData(Message) _returnvalue))
  (Class|IWeapon|IActivateWeaponHitbox(Message) (LocalVariables|GetTempWeapon) (.Damage (Utilities|Struct|BreakS_AttackDamageData (.Value (Utilities|Map|Find (Utilities|Struct|BreakS_ComboNameToDamageData (.Value (Utilities|Map|Find (Utilities|Struct|BreakS_AttackAnimationData _meleeattackanimationdata) (Animation|Montage|GetCurrentActiveMontage _returnvalue_2)))) (Animation|Montage|MontageGetCurrentSection _returnvalue_2 0))))) (.Knockback (Utilities|Struct|BreakS_AttackDamageData (.Value (Utilities|Map|Find (Utilities|Struct|BreakS_ComboNameToDamageData (.Value (Utilities|Map|Find (Utilities|Struct|BreakS_AttackAnimationData _meleeattackanimationdata) (Animation|Montage|GetCurrentActiveMontage _returnvalue_2)))) (Animation|Montage|MontageGetCurrentSection _returnvalue_2 0))))))
  (return false))
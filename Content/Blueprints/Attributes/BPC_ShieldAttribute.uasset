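; Shield attribute component that gives its owner a damage-absorbing shield with its own health.
; Init spawns a shield VFX actor attached to the owner's mesh, using settings from owner interface messages, and listens for its damage event.
; Hits trigger a timed, invulnerable hurt flash that reddens as health drops, plus drifting "ABSORB" text.
; At zero health it shows "BREAK!" and destroys the shield.
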(event Custom|OnShieldSpawned
  (Utilities|IsValid (Variables|Default|GetshieldVFX)
    (:Is%20Valid
      (Variables|Default|SetdefaultMaterial (Rendering|Material|GetMaterial (Variables|/Game/Blueprints/Attributes/BP_ShieldVFX.BP_ShieldVFX_C|GetShield (Variables|Default|GetshieldVFX)) 0))
      (EventDispatchers|BindEventtoOnDamageTaken (Variables|Default|GetshieldVFX) (delegate Custom|OnDamaged)))))

(event Custom|OnDamaged
  (params (damageAbsorbed :type Float%20%28single-precision%29))
  (if (not (Variables|Default|GetisHurt))
    (Variables|Default|SetisHurt true)
    (bind _output_get (Variables|Default|SetcurrHealth (- (Variables|Default|GetcurrHealth) damageAbsorbed)))
    (CallFunction|OnHurt)
    (if (<= _output_get 0.0)
      (CallFunction|SpawnStatusEffectMessage "BREAK!" "(R=0.666667,G=0.000000,B=0.008390,A=1.000000)")
      (CallFunction|KillShield)
      (else
        (CallFunction|SpawnStatusEffectMessage "ABSORB" (Variables|Default|GetflashTint))))))

(event Custom|OnHurt
  (Variables|Default|SetisHurt true)
  (Utilities|Time|SetTimerbyEvent (delegate Custom|FinishHurt) (Variables|Default|GethurtTime))
  (CallFunction|Flashon)
  (bind _returnvalue (Utilities|Time|SetTimerbyEvent (delegate Custom|ToggleFlash) (Variables|Default|GetFlashRate) true))
  (Variables|Default|SetFlashTimerHandle _returnvalue))

(event Custom|FinishHurt
  (Utilities|Time|PauseTimerbyHandle (Variables|Default|GetFlashTimerHandle))
  (CallFunction|FlashOff)
  (Variables|Default|SetisHurt false))

(event Custom|ToggleFlash
  (if (Variables|Default|GetIsFlashOn)
    (CallFunction|FlashOff)
    (else
      (CallFunction|Flashon))))

(fn Init
  (bind _shieldvfx (Variables|Default|GetshieldVFX))
  (Variables|Default|SetcurrHealth (Variables|Default|GetMaxHealth))
  (CallFunction|AddShieldVfX)
  (Variables|Default|SetisAlive true)
  (bind (_hurttime _flashrate) (Class|IPawn|IGetHurtData(Message) (Components|GetOwner)))
  (Variables|Default|SetFlashRate _flashrate)
  (Variables|Default|SethurtTime _hurttime)
  (Utilities|IsValid _shieldvfx
    (:Is%20Not%20Valid
      (bind _returnvalue (Rendering|Material|CreateDynamicMaterialInstance (Variables|/Game/Blueprints/Attributes/BP_ShieldVFX.BP_ShieldVFX_C|GetShield _shieldvfx) 0 (Variables|Default|GethurtMat) "None" :!class /Script/Engine.PrimitiveComponent))
      (Rendering|Material|GetVectorParameterValue _returnvalue "FlashCol" :!class /Script/Engine.MaterialInstanceDynamic))))

(fn IsShieldAlive
  (return (Variables|Default|GetisAlive)))

(fn AddShieldVfX
  (bind (_scale _spawnoffset) (Class|IElite|GetShieldVFXSettings(Message) (Components|GetOwner)))
  (bind _skeletalmesh (Class|IPawn|IGetMesh(Message) (Components|GetOwner)))
  (bind _output_get (Variables|Default|SetcharacterMesh _skeletalmesh))
  (bind _output_get_2 (Variables|Default|SetshieldOffset _spawnoffset))
  (bind _returnvalue (Game|SpawnActorfromClass "/Game/Blueprints/Attributes/BP_ShieldVFX.BP_ShieldVFX_C" (Math|Transform|MakeTransform (+ _output_get_2 (Transformation|GetWorldLocation _output_get)) "0, 0, 0" _scale) "Undefined" 0 0))
  (Variables|Default|SetshieldVFX _returnvalue)
  (Transformation|AttachComponentToComponent (Variables|Default|GetshieldVFX) (Variables|Default|GetcharacterMesh) "None" "KeepWorld" "KeepWorld" "KeepWorld" true)
  (CallFunction|OnShieldSpawned))

(fn KillShield
  (bind _shieldvfx (Variables|Default|GetshieldVFX))
  (Variables|Default|SetisAlive false)
  (Utilities|IsValid _shieldvfx
    (:Is%20Valid
      (Actor|DestroyActor _shieldvfx))))

(fn Flashon
  (bind _shieldvfx (Variables|Default|GetshieldVFX))
  (bind _maxhealth (Variables|Default|GetMaxHealth))
  (bind _currhealth (Variables|Default|GetcurrHealth))
  (bind _returnvalue (/ _currhealth _maxhealth))
  (Utilities|IsValid _shieldvfx
    (:Is%20Valid
      (bind _returnvalue_2 (Rendering|Material|CreateDynamicMaterialInstance (Variables|/Game/Blueprints/Attributes/BP_ShieldVFX.BP_ShieldVFX_C|GetShield _shieldvfx) 0 (Variables|Default|GethurtMat) "None" :!class /Script/Engine.PrimitiveComponent))
      (bind _returnvalue_3 (Rendering|Material|GetVectorParameterValue _returnvalue_2 "FlashCol" :!class /Script/Engine.MaterialInstanceDynamic))
      (bind _output_get (LocalVariables|SetFlashColour _returnvalue_3))
      (bind _output_get_2 (Variables|Default|SetflashTint (Utilities|Struct|MakeLinearColor (/ (.r _output_get) _returnvalue) (* (.g _output_get) _returnvalue) (* (.b _output_get) _returnvalue) (.a _output_get))))
      (Rendering|Material|SetVectorParameterValue _returnvalue_2 "FlashCol" _output_get_2 :!class /Script/Engine.MaterialInstanceDynamic)
      (Variables|Default|SetIsFlashOn true))))

(fn FlashOff
  (bind _shieldvfx (Variables|Default|GetshieldVFX))
  (Utilities|IsValid _shieldvfx
    (:Is%20Valid
      (Rendering|Material|CreateDynamicMaterialInstance (Variables|/Game/Blueprints/Attributes/BP_ShieldVFX.BP_ShieldVFX_C|GetShield _shieldvfx) 0 (Variables|Default|GetdefaultMaterial) "None" :!class /Script/Engine.PrimitiveComponent)
      (Variables|Default|SetIsFlashOn false))))

(fn SpawnStatusEffectMessage
  (params (statusText :type String) (textColour :type Linear%20Color%20Structure))
  (bind _returnvalue (Components|GetOwner))
  (bind _returnvalue_2 (Transformation|GetActorLocation _returnvalue))
  (bind (_x _y _z) (Math|Vector|BreakVector _returnvalue_2))
  (bind _point (Class|IPawn|IRandomPointinSphere(Message) (Components|GetOwner) (Math|Vector|MakeVector _x _y (+ _z 1e+02 0.0)) 2e+02))
  (LocalVariables|Setrand%20point _point)
  (LocalVariables|Setdir (Math|Vector|GetUnitDirection(Vector) (Transformation|GetActorLocation (Components|GetOwner)) (LocalVariables|Getrand%20point)))
  (Game|SpawnActorfromClass "/Game/Blueprints/VFX/BP_DamageTypeText.BP_DamageTypeText_C" (Math|Transform|MakeTransform (Transformation|GetActorLocation (Components|GetOwner)) "0, 0, 0" "1,1,1") "Undefined" 0 statusText 3.5 0.0 textColour (LocalVariables|Getdir) 0.0 0))
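; BPC_StatusEffectAttribute is a component that adds a status effect, currently only toxin, to the attacks of its owner's weapon.
; Init stores the effect type; for Toxin it packs duration, tick rate and damage range, binds to the weapon's attack event and enables its VFX.
; Each attack passes that data, the owner and its location to the target through an ApplyToxicDamage message.
; Disable is an empty stub.
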(event Custom|OnSetUpToxin
  (Variables|Default|SettoxicData (Utilities|Struct|MakeS_ToxinData (Variables|Default|GetToxinDuration) (Variables|Default|GetPoisonTickRate) (Variables|Default|GetminDMGperTick) (Variables|Default|GetmaxDmgPerTIck)))
  (bind _weapon (Class|ICharacter|GetWeapon(Message) (Components|GetOwner)))
  (EventDispatchers|BindEventtoOnAttack _weapon (delegate Custom|ApplyToxin))
  (Default|EnableStatusEffectVFX _weapon (Variables|Default|GetactiveEffect)))

(event Custom|ApplyToxin
  (params (target :type Actor%20Object%20Reference))
  (bind _returnvalue (Components|GetOwner))
  (Class|IDamageable|ApplyToxicDamage(Message) target _returnvalue (Transformation|GetActorLocation _returnvalue) (Variables|Default|GettoxicData)))

(fn Init
  (params (satusEffectType :type E_StatusEffect%20Enum :default "NewEnumerator0"))
  (bind _output_get (Variables|Default|SetactiveEffect satusEffectType))
  (Variables|Default|Setenabled true)
  (switch Utilities|FlowControl|Switch|SwitchonE_StatusEffect _output_get
    (:NewEnumerator1
      (CallFunction|OnSetUpToxin))))

(fn Disable)
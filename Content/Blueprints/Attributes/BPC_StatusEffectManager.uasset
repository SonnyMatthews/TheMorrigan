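; Actor component that manages poison and stun status effects on its owner, reaching it through interface messages.
; Poison runs a looping timer that deals random damage with floating "POISON" text until a duration timer ends it.
; Stun notifies the owner on start and end, then blocks re-stunning for a cooldown.
; Particle emitters are reused once spawned, and Tick moves active ones to the mesh's Neck socket.
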(event Custom|OnAddToxicDamage
  (params (toxin :type S%20Toxin%20Data%20Structure))
  ;[1 1 1] On Apply toxin
  (if (not (Variables|States|GetisPoisoned))
    (CallFunction|AddToxinEffect)
    (Variables|States|SetisPoisoned true)
    (bind _output_get (Variables|Settings|SetCurrentToxinData toxin))
    (bind _returnvalue (Utilities|Time|SetTimerbyEvent (delegate Custom|OnApplyToxic) (.tickrate _output_get) true (.tickrate _output_get)))
    (Variables|Settings|SetToxinTimer _returnvalue)
    (Utilities|Time|SetTimerbyEvent (delegate Custom|ToxinRanOut) (.duration (Variables|Settings|GetCurrentToxinData)))))

(event Custom|EndStun
  ;[1 1 1] OnApplyStun
  (Variables|States|SetisStunned false)
  (Class|IStatusEffects|OnRemoveStun(Message) (Components|GetOwner))
  (Utilities|Time|SetTimerbyEvent (delegate Custom|OnEndStunImmunity) (Variables|Settings|GetstunCooldown)))

(event Custom|ToxinRanOut
  ;[1 1 1] On Apply toxin
  (Variables|States|SetisPoisoned false)
  (Utilities|Time|PauseTimerbyHandle (Variables|Settings|GetToxinTimer))
  (CallFunction|ClearToxin))

(event Custom|OnApplyStun
  (params (StunTime :type Float%20%28single-precision%29))
  ;[1 1 1] OnApplyStun
  (Variables|Settings|SetStunTime StunTime)
  (if (and (Variables|States|GetcanBeStunned) (not (Variables|States|GetisStunned)))
    (Variables|States|SetisStunned true)
    (Variables|States|SetcanBeStunned false)
    (CallFunction|AddStun)
    (Utilities|Time|SetTimerbyEvent (delegate Custom|EndStun) (Variables|Settings|GetStunTime))))

(event Custom|OnApplyToxic
  (bind _currenttoxindata (Variables|Settings|GetCurrentToxinData))
  ;[1 1 1] On Apply toxin
  (Class|IDamageable|Damage(Message) (Components|GetOwner) (Math|Random|RandomFloatinRange (.mindamagepertick _currenttoxindata) (.maxdamagepertick _currenttoxindata)) 0.0 0 "0, 0, 0")
  (CallFunction|SpawnStatusEffectDmg "(R=0.097587,G=0.822786,B=0.054480,A=1.000000)" "POISON")
  (if (not (Variables|States|GetisPoisoned))
    (Utilities|Time|PauseTimerbyHandle (Variables|Settings|GetToxinTimer))))

(event Custom|OnEndStunImmunity
  ;[1 1 1] OnApplyStun
  (Variables|States|SetcanBeStunned true))

(event EventBeginPlay)

(event EventTick
  (params (DeltaSeconds :type Float%20%28single-precision%29))
  (bind _stunvfx (Variables|Default|GetStunVFX))
  (bind _toxineffect (Variables|Default|GettoxinEffect))
  (bind _stunvfx_2 (Variables|Default|GetStunVFX))
  (bind _toxineffect_2 (Variables|Default|GettoxinEffect))
  ;[1 1 1] OnTick
  (if (Variables|States|GetisPoisoned)
    (Utilities|IsValid _toxineffect_2
      (:Is%20Valid
        (CallFunction|UpdateEffectPosition _toxineffect_2)
        (if (Variables|States|GetisStunned)
          (Utilities|IsValid _stunvfx
            (:Is%20Valid
              (CallFunction|UpdateEffectPosition _stunvfx))))))
    (elif (Variables|States|GetisStunned)
      (Utilities|IsValid _stunvfx_2
        (:Is%20Valid
          (CallFunction|UpdateEffectPosition _stunvfx_2)
          (if (Variables|States|GetisPoisoned)
            (Utilities|IsValid _toxineffect
              (:Is%20Valid
                (CallFunction|UpdateEffectPosition _toxineffect)))))))))

(fn ClearToxin
  (bind _toxineffect (Variables|Default|GettoxinEffect))
  (Utilities|IsValid _toxineffect
    (:Is%20Valid
      (Components|Activation|Deactivate _toxineffect))))

(fn ClearStun
  (bind _stunvfx (Variables|Default|GetStunVFX))
  (Utilities|IsValid _stunvfx
    (:Is%20Valid
      (Components|Activation|Deactivate _stunvfx))))

(fn AddToxinEffect
  (bind _skeletalmesh (Class|IPawn|IGetMesh(Message) (Components|GetOwner)))
  (Utilities|IsValid (Variables|Default|GettoxinEffect)
    (:Is%20Valid
      (Components|Activation|Activate (Variables|Default|GettoxinEffect) true))
    (:Is%20Not%20Valid
      (bind _returnvalue (Effects|SpawnEmitteratLocation "/Game/ParticleSystem/P_PoisonMist.P_PoisonMist" (Transformation|GetSocketLocation _skeletalmesh "Neck") "0, 0, 0" "0.100000,0.100000,0.100000"))
      (Variables|Default|SettoxinEffect _returnvalue))))

(fn UpdateEffectPosition
  (params (effect :type Scene%20Component%20Object%20Reference))
  (bind _skeletalmesh (Class|IPawn|IGetMesh(Message) (Components|GetOwner)))
  (Transformation|SetWorldLocation effect (Transformation|GetSocketLocation _skeletalmesh "Neck") false false))

(fn SpawnStatusEffectDmg
  (params (textColour :type Linear%20Color%20Structure) (statusText :type String))
  (bind _returnvalue (Components|GetOwner))
  (bind _returnvalue_2 (Transformation|GetActorLocation _returnvalue))
  (bind (_x _y _z) (Math|Vector|BreakVector _returnvalue_2))
  (bind _point (Class|IPawn|IRandomPointinSphere(Message) (Components|GetOwner) (Math|Vector|MakeVector _x _y (+ _z 1e+02)) 3e+01))
  (LocalVariables|Setrand%20point _point)
  (LocalVariables|Setdir (Math|Vector|GetUnitDirection(Vector) (Transformation|GetActorLocation (Components|GetOwner)) (LocalVariables|Getrand%20point)))
  (Game|SpawnActorfromClass "/Game/Blueprints/VFX/BP_DamageTypeText.BP_DamageTypeText_C" (Math|Transform|MakeTransform (Transformation|GetActorLocation (Components|GetOwner)) "0, 0, 0" "1,1,1") "Undefined" 0 statusText 3.0 0.0 textColour (LocalVariables|Getdir) 0.0 0))

(fn AddStun
  (bind _skeletalmesh (Class|IPawn|IGetMesh(Message) (Components|GetOwner)))
  (Utilities|IsValid (Variables|Default|GetStunVFX)
    (:Is%20Valid
      (Components|Activation|Activate (Variables|Default|GetStunVFX) true)
      (Class|IStatusEffects|OnStun(Message) (Components|GetOwner)))
    (:Is%20Not%20Valid
      (bind _returnvalue (Effects|SpawnEmitteratLocation "/Game/InfinityBladeEffects/Effects/FX_Ability/Stun/P_Stun_Stars_Base.P_Stun_Stars_Base" (Transformation|GetSocketLocation _skeletalmesh "Neck")))
      (Variables|Default|SetStunVFX _returnvalue)
      (Class|IStatusEffects|OnStun(Message) (Components|GetOwner)))))
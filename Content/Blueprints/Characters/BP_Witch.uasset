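; Witch enemy character that switches between idle, wander, chase, melee and spell attack states, extending a parent AI character.
; State changes notify listeners and run the matching behavior, while Tick turns the witch toward its target in attack states.
; Spell casting halts movement, scales up a child-actor VFX on a timeline, then spawns a projectile configured from a data table.
; AI data rows set detection radius, health and default state.
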(event Custom|BeginAttackSpell
  (bind _spelldata (Variables|AIData|GetSpellData))
  (bind _castingpoint (Variables|Default|GetCastingPoint))
  (bind _castingpoint_2 (Variables|Default|GetCastingPoint))
  (bind _castingpoint_3 (Variables|Default|GetCastingPoint))
  ;[1 1 1] If already channelling spell don't  start again
  (if (not (Variables|AttackSettings|GetIsChannelling))
    (Variables|AttackSettings|SetIsChannelling true)
    ;[1 1 1] Initialise casting anim
    (Transformation|SetWorldScale3D _castingpoint "0, 0, 0")
    (ChildActorComponent|SetChildActorClass _castingpoint (Variables|Default|GetSpellVFX))
    (bind _channelcurve (Timeline|ChannelTimeLine PlayFromStart)
      (:Update
        (Transformation|SetWorldScale3D _castingpoint_3 (Math|Vector|Lerp(Vector) (Transformation|GetWorldScale _castingpoint_3) (Variables|Default|GetMaxSpellVFXScale) _channelcurve)))
      (:Finished
        (Utilities|FlowControl|Delay 0.5)
        (ChildActorComponent|SetChildActorClass (Variables|Default|GetCastingPoint) 0)
        (Game|SpawnActorfromClass (Variables|Default|GetSpell) (Math|Transform|MakeTransform (Transformation|GetWorldLocation _castingpoint_2) (Math|Rotator|MakeRotfromX (Math|Vector|GetForwardVector _castingpoint_2)) "1,1,1") "Undefined" 0 (.projectiledamage _spelldata) (.projectilestartspeed _spelldata) (.projectilemaxspeed _spelldata) (.gravity _spelldata) (.lifespan _spelldata) (.maxenemycanhit _spelldata) (Transformation|GetWorldScale _castingpoint_2) 0)
        (Variables|AttackSettings|SetIsChannelling false)))))

(event EventBeginPlay
  ;[1 1 1] Begin
  (|CallParentFunction)
  (CallFunction|SetSpellData (Variables|AIData|GetSpellDT) (Variables|AIData|GetSpellName))
  (ChildActorComponent|SetChildActorClass (Variables|Default|GetCastingPoint) 0)
  (Variables|Default|SetMaxSpellVFXScale (Transformation|GetWorldScale (Variables|Default|GetCastingPoint))))

(event EventUpdateWitchState
  (params (NewState :type E_WitchState%20Enum :default "NewEnumerator0"))
  (CallFunction|SetWitchState NewState))

(event EventTick
  (params (DeltaSeconds :type Float%20%28single-precision%29))
  ;[1 1 1] Event Tick
  ;;[1 0.9188 0.09302] While channelig a spell or in attack mode rotate to face palyer
  (Utilities|SwtichState
    (:MeleeAttack
      _)
    (:SpellAttack
      _))
  (if (not (Variables|Default|GetIsAttacking))
    (Utilities|IsValid (Variables|Default|GetcurrentTarget)
      (:Is%20Valid
        (Transformation|SetActorRotation (Math|Rotator|MakeRotator 0.0 0.0 (.yaw (Math|Interpolation|RInterpTo (Transformation|GetActorRotation) (Math|Rotator|FindLookatRotation (Transformation|GetActorLocation) (Transformation|GetActorLocation (Variables|Default|GetcurrentTarget))) DeltaSeconds 0.5))))))))

(event EventTargetDestroyed
  (CallFunction|SetWitchState (Variables|AIData|GetDefaultWitchState)))

(fn ConstructionScript
  (|CallParentFunction))

(fn InitAttack
  (|CallParentFunction))

(fn EvaluateCurrentState
  (Utilities|SwtichState
    (:Idle
      (CallFunction|InitIdle)
      (Variables|AttackSettings|SetIsChannelling false :!label _label))
    (:Wander
      (CallFunction|InitWander)
      (goto _label))
    (:MeleeAttack
      (CallFunction|InitAttack)
      (goto _label))
    (:Chase
      (CallFunction|InitChase)
      (goto _label))
    (:SpellAttack
      (CallFunction|BeginAttackSpell)
      (Variables|/Script/Engine.CharacterMovementComponent|SetMaxWalkSpeed (Variables|Character|GetCharacterMovement) 0.0))))

(fn SetSpellData
  (params (DataTable :type Data%20Table%20Object%20Reference) (RowName :type Name))
  (bind _returnvalue (Utilities|GetDataTableRow DataTable RowName)
    (:then
      (Variables|AIData|SetSpellData _returnvalue))))

(fn GetWitchData
  (bind _aidata (Variables|Default|GetAIData))
  (return (.attackrange _aidata) (.wanderrange _aidata) (.closecombatrange _aidata) (.wanderwaittime _aidata) (Variables|AIData|GetDefaultWitchState) (Variables|AIData|GetWitchStates) (Variables|Default|GetcurrentTarget)))

(fn SetAIData
  (params (DataTable :type Data%20Table%20Object%20Reference) (RowName :type Name :default "None"))
  (bind _returnvalue (Utilities|GetDataTableRow DataTable RowName)
    (:then
      (bind _output_get (Variables|Default|SetAIData _returnvalue))
      (bind _structout (Utilities|Struct|SetmembersinS_AIData _output_get))
      (Components|Sphere|SetSphereRadius (Variables|Default|GetVisionArea) (.detectionrange _structout) false)
      (Variables|Default|SetCurrentHealth (.maxhealth _structout))
      (if (< (Math|Conversions|ToInteger(Byte) (.defaultaistate _structout)) 4)
        (Variables|AIData|SetDefaultWitchState (Utilities|Enum|ByteToEnumE_WitchState (Math|Conversions|ToByte(Integer) (Math|Conversions|ToInteger(Byte) (.defaultaistate _structout)))))
        (else
          (Variables|AIData|SetDefaultWitchState "NewEnumerator1"))))))

(fn SetWitchState
  (params (NewWitchState :type E_WitchState%20Enum :default "NewEnumerator0"))
  (bind _output_get (Variables|AIData|SetWitchStates NewWitchState))
  (Default|CallOnNewWitchState _output_get)
  (CallFunction|EvaluateCurrentState))
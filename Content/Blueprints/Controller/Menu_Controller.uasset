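; Menu_Controller is a player controller that shows the main menu and routes navigation input to it.
; On BeginPlay it creates a W_MainMenu widget, stores it and adds it to the viewport.
; Up and left shoulder presses send one navigation enum value to the widget's ReceiveNavInput, while down and right shoulder presses send the other.
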(event EventBeginPlay
  (bind _returnvalue (UserInterface|CreateWidget "/Game/Blueprints/Widgets/W_MainMenu.W_MainMenu_C" self))
  (Variables|Default|SetMain_Menu _returnvalue)
  (UserInterface|Viewport|AddtoViewport _returnvalue 0))

(event EventTick
  (params (DeltaSeconds :type Float%20%28single-precision%29)))

(event Input|ActionEvents|InputActionUpUI
  (params (Key :type Key%20Structure :default "None"))
  (:Pressed
    (Default|ReceiveNavInput (Variables|Default|GetMain_Menu) "NewEnumerator1")))

(event Input|ActionEvents|InputActionDownUI
  (params (Key :type Key%20Structure :default "None"))
  (:Pressed
    (Default|ReceiveNavInput (Variables|Default|GetMain_Menu) "NewEnumerator0")))

(event Input|ActionEvents|InputActionRightShoulderUI
  (params (Key :type Key%20Structure :default "None"))
  (:Pressed
    (Default|ReceiveNavInput (Variables|Default|GetMain_Menu) "NewEnumerator0")))

(event Input|ActionEvents|InputActionLeftShoulderUI
  (params (Key :type Key%20Structure :default "None"))
  (:Pressed
    (Default|ReceiveNavInput (Variables|Default|GetMain_Menu) "NewEnumerator1")))

(fn ConstructionScript)
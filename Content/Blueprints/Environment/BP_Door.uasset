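; BP_Door is a door that sinks downward when triggered, with a short camera cutaway to show it opening.
; ITrigger slows the player pawn through custom time dilation, blends the view to the door, then a timeline lerps the Cube down after a delay.
; After a pause, the view blends back to BP_Char_Player and normal pawn speed returns.
; IReset snaps the Cube back to the location saved at BeginPlay.
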(event EventIReset
  (Transformation|SetWorldLocation (Variables|Default|GetCube) (Variables|Default|GetSpawnLoc) false false))

(event EventBeginPlay
  (Variables|Default|SetSpawnLoc (Transformation|GetWorldLocation (Variables|Default|GetCube))))

(event EventITrigger
  (bind _returnvalue (Game|GetPlayerController 0))
  (bind _returnvalue_2 (Game|GetPlayerController 0))
  (bind _cube (Variables|Default|GetCube))
  (bind _returnvalue_3 (Transformation|GetWorldLocation _cube))
  (Variables|/Script/Engine.Actor|SetCustomTimeDilation (Pawn|GetControlledPawn _returnvalue_2) 0.2)
  (Game|Player|SetViewTargetwithBlend _returnvalue_2 self 1.0 "VTBlend_Linear" 0.0 false)
  (Utilities|FlowControl|Delay 2.0)
  (Variables|Default|SetStartLoc _returnvalue_3)
  (Variables|Default|SetTargetLoc (- _returnvalue_3 "0, 0,300.000000"))
  (bind _newtrack_2 (Timeline|Timeline_0 PlayFromStart)
    (:Update
      (Transformation|SetWorldLocation (Variables|Default|GetCube) (Math|Vector|Lerp(Vector) (Variables|Default|GetStartLoc) (Variables|Default|GetTargetLoc) _newtrack_2) false false))
    (:Finished
      (Utilities|FlowControl|Delay 2.0)
      (bind _asbp_char_player (Utilities|Casting|CastToBP_Char_Player (Pawn|GetControlledPawn _returnvalue)))
      (Game|Player|SetViewTargetwithBlend _returnvalue _asbp_char_player 1.0 "VTBlend_Linear" 0.0 false)
      (Variables|/Script/Engine.Actor|SetCustomTimeDilation (Pawn|GetControlledPawn _returnvalue) 1.0))))

(fn ConstructionScript)
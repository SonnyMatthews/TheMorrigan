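; BP_SpawnTrigger is a one-shot trigger volume that signals its AreaEnemyManager when the player enters.
; The box overlap filters for BP_Char_Player and passes through a DoOnce gate, which sends ITriggerMessage to the manager.
; On BeginPlay it binds to the game mode's new-state event, and the Init Player Respawn state calls IReset to re-arm the gate.
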(event OnComponentBeginOverlap(Box)
  (params (OverlappedComponent :type Primitive%20Component%20Object%20Reference) (OtherActor :type Actor%20Object%20Reference) (OtherComp :type Primitive%20Component%20Object%20Reference) (OtherBodyIndex :type Integer) (bFromSweep :type Boolean) (SweepResult :type Hit%20Result%20Structure%20%28by%20ref%29))
  (if (== (Utilities|GetClass OtherActor) "/Game/Blueprints/Pawn/BP_Char_Player.BP_Char_Player_C")
    (Utilities|FlowControl|DoOnce false
      (:Completed
        (Class|ITrigger|ITrigger(Message) (Variables|Default|GetAreaEnemyManager))))))

(event Custom|OnNewGameState
  (params (NewState :type E_GameStates%20Enum :default "NewEnumerator0"))
  (switch Utilities|FlowControl|Switch|SwitchonE_GameStates NewState
    (:NewEnumerator10
      (CallFunction|IReset))))

(event Custom|OnBindToGameMode
  (bind _gamemode (Class|IMorriganGameMode|GetGameModeRef(Message) (Game|GetGameMode)))
  (EventDispatchers|BindEventtoOnNewState _gamemode (delegate Custom|OnNewGameState)))

(event EventBeginPlay
  (CallFunction|OnBindtoGameMode))

(event Collision|EventActorBeginOverlap
  (params (OtherActor :type Actor%20Object%20Reference)))

(event EventTick
  (params (DeltaSeconds :type Float%20%28single-precision%29)))

(event EventIReset
  (Utilities|FlowControl|DoOnce false) ; enters at Reset
)

(fn ConstructionScript)
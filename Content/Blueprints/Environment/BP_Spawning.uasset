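; BP_Spawning is a one-shot enemy spawn point that creates an enemy at its own transform after a configurable delay.
; On BeginPlay it switches on EnemyType, destroying itself immediately when Blank.
; Melee and Ranged currently both spawn BP_BaseEnemy, pass the new enemy out through CallReference, then destroy the spawner a second later.
; A comment marks the BeginPlay logic for replacement with an Init.
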(event EventBeginPlay
  (bind _returnvalue (Transformation|GetActorTransform))
  ;[1 1 1] Replace with Init
  (if (Utilities|Enum|Equal(Enum) (Variables|Default|GetEnemy%20Type) "NewEnumerator4")
    (Actor|DestroyActor :!label _label)
    (else
      (Utilities|FlowControl|Delay (Variables|Default|GetSpawn%20Delay))
      (switch Utilities|FlowControl|Switch|SwitchonEnum_EnemyType (Variables|Default|GetEnemy%20Type)
        (:NewEnumerator4
          (goto _label))
        (:NewEnumerator0
          (bind _returnvalue_2 (Game|SpawnActorfromClass "/Game/Blueprints/AI/Characters/BP_BaseEnemy.BP_BaseEnemy_C" _returnvalue "Undefined" 0 0))
          (Default|CallReference _returnvalue_2)
          (Utilities|FlowControl|Delay 1.0)
          (Actor|DestroyActor))
        (:NewEnumerator3
          (bind _returnvalue_3 (Game|SpawnActorfromClass "/Game/Blueprints/AI/Characters/BP_BaseEnemy.BP_BaseEnemy_C" _returnvalue "Undefined" 0 0))
          (Default|CallReference _returnvalue_3)
          (Utilities|FlowControl|Delay 1.0)
          (Actor|DestroyActor))))))

(event Collision|EventActorBeginOverlap
  (params (OtherActor :type Actor%20Object%20Reference)))

(event EventTick
  (params (DeltaSeconds :type Float%20%28single-precision%29)))

(fn ConstructionScript)
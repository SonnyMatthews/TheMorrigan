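; Level exit actor that ends the level when the player reaches it.
; When triggered through ITrigger (or on BeginPlay in debug), it spawns a particle effect and enables its box collision.
; On player pawn overlap, unless IsGameEnd is set, it switches controls, creates the level-end widget with TargetLevel and saves via the game mode.
; The game mode's blackout event removes that widget.
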(event OnComponentBeginOverlap(Box)
  (params (OverlappedComponent :type Primitive%20Component%20Object%20Reference) (OtherActor :type Actor%20Object%20Reference) (OtherComp :type Primitive%20Component%20Object%20Reference) (OtherBodyIndex :type Integer) (bFromSweep :type Boolean) (SweepResult :type Hit%20Result%20Structure%20%28by%20ref%29))
  (bind _returnvalue (Game|GetPlayerController 0))
  (bind _targetlevel (Variables|Default|GetTargetLevel))
  (if (not (Variables|Default|GetisGameEnd))
    (if (== OtherActor (Game|Player|GetPlayerPawn 0))
      (Class|IControllerUI|SetNewGameControl(Message) _returnvalue "NewEnumerator1" false)
      (Variables|/Script/Engine.PlayerController|SetbShowMouseCursor _returnvalue true)
      (bind _returnvalue_2 (UserInterface|CreateWidget "/Game/Blueprints/UI/Widget_LevelEnd.Widget_LevelEnd_C"))
      (bind _output_get (Variables|Default|SetendLevelScreen _returnvalue_2))
      (UserInterface|Viewport|AddtoViewport _output_get 0)
      (Default|InitNextLevel (Variables|Default|GetendLevelScreen) _targetlevel)
      (bind _gamemode (Class|IMorriganGameMode|GetGameModeRef(Message) (Game|GetGameMode)))
      (Default|SaveGame _gamemode _targetlevel))))

(event Custom|RemoveEndLevelScreen
  (Utilities|IsValid (Variables|Default|GetendLevelScreen)
    (:Is%20Valid
      (Widget|RemovefromParent (Variables|Default|GetendLevelScreen)))))

(event EventBeginPlay
  (bind _gamemode (Class|IMorriganGameMode|GetGameModeRef(Message) (Game|GetGameMode)))
  (EventDispatchers|BindEventtoOnBlackOut _gamemode (delegate Custom|RemoveEndLevelScreen))
  (if (Variables|Default|GetinDebug)
    (CallFunction|ITrigger)))

(event EventITrigger
  (bind _returnvalue (Effects|SpawnEmitterAttached (Variables|Default|GetParticle%20Effect) (Variables|Default|GetBox) "None" "0, 0, 0" "0, 0, 0" "0.150000,0.150000,0.150000"))
  (Variables|Default|SetEmitter _returnvalue)
  (Collision|SetCollisionEnabled (Variables|Default|GetBox) "QueryAndPhysics"))

(fn ConstructionScript)
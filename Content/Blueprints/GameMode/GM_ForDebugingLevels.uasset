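; Debug game mode for testing levels, setting up a playable character and sound manager without further game flow.
; PostLogin shows the cursor, spawns BP_SoundManager, then spawns and possesses a BP_Char_Player at every PlayerStart, resetting stats through the GameInstance.
; A one-second delay precedes the character's init message and HUD display.
; GetSoundManager exposes the manager, while GetGameModeRef and GetGameState are empty stubs.
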(event EventPostLogin
  (params (NewPlayer :type Player%20Controller%20Object%20Reference))
  (bind _returnvalue (Game|GetGameInstance))
  (bind _output_get (Variables|Default|SetP_Controller NewPlayer))
  (Variables|/Script/Engine.PlayerController|SetbShowMouseCursor _output_get true)
  (bind _returnvalue_2 (Game|SpawnActorfromClass "/Game/Blueprints/Managers/BP_SoundManager.BP_SoundManager_C" (Math|Transform|MakeTransform "0, 0, 0") "Undefined" 0 0))
  (Variables|Default|SetSoundManager _returnvalue_2)
  (bind _outactors (Actor|GetAllActorsOfClass "/Script/Engine.PlayerStart"))
  (for _array_element _outactors
    (bind _returnvalue_3 (Game|SpawnActorfromClass "/Game/Blueprints/Pawn/BP_Char_Player.BP_Char_Player_C" (Transformation|GetActorTransform _array_element) "Undefined" 0 0))
    (Class|IInstance|SetPlayerDefaultStats(Message) _returnvalue "Iter1")
    (Class|IInstance|ResetPlayerStats(Message) _returnvalue)
    (Pawn|Possess (Variables|Default|GetP_Controller) _returnvalue_3)
    (Utilities|FlowControl|Delay 1.0)
    (Class|IInitialisable|Init(Message) _returnvalue_3)
    (Default|ToggleHUD _returnvalue_3 true)))

(fn ConstructionScript)

(fn GetGameModeRef)

(fn GetGameState)

(fn GetSoundManager
  (return (Variables|Default|GetSoundManager)))
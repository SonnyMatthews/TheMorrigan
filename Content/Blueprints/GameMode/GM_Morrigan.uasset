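; Game mode for Morrigan that runs the game flow from startup through level loading, player spawning, death and respawn.
; An event-dispatched state machine (NewState) chains init, level-instance streaming, character spawn and possession, spawn-point lookup by parent level, and UI setup.
; Screen-fade completion callbacks gate transitions and the delayed respawn at the active spawn point.
; It also spawns the sound manager and recreates the local player at init.
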(event Custom|NewState
  (params (NewState :type E_GameStates%20Enum :default "NewEnumerator0"))
  (switch Utilities|FlowControl|Switch|SwitchonE_GameStates NewState
    (:NewEnumerator0
      (EventDispatchers|BindEventtoOnAllLevelsUnloaded (delegate Custom|InitLevel))
      (CallFunction|InitGameMode))
    (:NewEnumerator14
      (CallFunction|LoadNextLevel (Variables|Default|GetTargetLevel)))
    (:NewEnumerator5
      (CallFunction|SetUpCharacter))
    (:NewEnumerator4
      (EventDispatchers|BindEventtoOnFadeComplete (Variables|Default|GetfadeWidget) (delegate Custom|OnTransitioEnd))
      (CallFunction|EndTransition))
    (:NewEnumerator13
      (CallFunction|GetActiveSpawn))
    (:NewEnumerator12
      (CallFunction|SpawnPlayer))
    (:NewEnumerator15
      (CallFunction|InitUI))
    (:NewEnumerator9
      (CallFunction|DisablePlayerUI))
    (:NewEnumerator10
      (Variables|Default|SetCurrentGameState "NewEnumerator10")
      (CallFunction|RespawnPlayer))
    (:NewEnumerator11
      (Variables|Default|SetCurrentGameState "NewEnumerator11")
      (EventDispatchers|BindEventtoOnFadeComplete (Variables|Default|GetfadeWidget) (delegate Custom|OnRespawnTransEnd))
      (Default|ResetPlayer (Variables|Default|GetPlayerCharacter))
      (CallFunction|EndTransition))))

(event Custom|Respawn
  (bind _currentspawnpoint (Variables|Default|GetcurrentSpawnPoint))
  ;[1 1 1] Respawn
  (Utilities|IsValid _currentspawnpoint
    (:Is%20Valid
      (bind _spawnpoint (Default|GetSpawnPoint _currentspawnpoint))
      (Transformation|SetActorLocation (Variables|Default|GetPlayerCharacter) _spawnpoint false false)
      (Transformation|SetActorRotation (Variables|Default|GetPlayerCharacter) (Transformation|GetActorRotation _currentspawnpoint)))))

(event Custom|OnTransitioEnd
  (EventDispatchers|UnbindEventfromOnFadeComplete (Variables|Default|GetfadeWidget) (delegate Custom|OnTransitioEnd))
  (Default|SetCamLagSpeed (Variables|Default|GetPlayerCharacter) true 0.0)
  (Default|CallOnNewState "NewEnumerator15"))

(event Custom|Respawn%20Binding
  ;[1 1 1] Resets Rooms when player is destroyed
  (EventDispatchers|BindEventtoPlayerDied (Variables|Default|GetPlayerCharacter) (delegate Custom|Player%20Died)))

(event Custom|Player%20Died
  ;[1 1 1] Resets Rooms when player is destroyed
  (Variables|Default|SetCurrentGameState "NewEnumerator9")
  (Default|CallOnNewState "NewEnumerator9")
  (EventDispatchers|BindEventtoOnFadeComplete (Variables|Default|GetfadeWidget) (delegate Custom|OnDeathTransEnd))
  (Default|OnFadein (Variables|Default|GetfadeWidget)))

(event Custom|OnUnloadLevel
  (params (Level%20Name :type String))
  ;[1 1 1] On Unload Level
  (if (Class|LevelStreaming|IsLevelLoaded (Class|GameplayStatics|GetStreamingLevel (Utilities|String|StringToName Level%20Name)))
    (Game|UnloadStreamLevel(byName) (Utilities|String|StringToName Level%20Name) false)
    (Default|CallOnLevelUnloaded)))

(event Custom|InitLevel
  (EventDispatchers|UnbindEventfromOnAllLevelsUnloaded (delegate Custom|InitLevel))
  (Default|CallOnNewState "NewEnumerator14"))

(event Custom|OnRespawnTransEnd
  (EventDispatchers|UnbindEventfromOnFadeComplete (Variables|Default|GetfadeWidget) (delegate Custom|OnRespawnTransEnd))
  (Default|SetCamLagSpeed (Variables|Default|GetPlayerCharacter) true 0.0)
  (Default|CallOnNewState "NewEnumerator15"))

(event Custom|BindToLevelLoaded
  (params (LevelPackage :type Level%20Streaming%20Object%20Reference))
  ;[1 1 1] On Level Loaded
  (Variables|Default|SetcurrLevelStream LevelPackage)
  (EventDispatchers|BindEventtoOnLevelLoaded LevelPackage (delegate Custom|OnLevelLoaded)))

(event Custom|OnLevelLoaded
  ;[1 1 1] On Level Loaded
  (Utilities|IsValid (Variables|Default|GetcurrLevelStream)
    (:Is%20Valid
      (if (Class|LevelStreaming|IsLevelLoaded (Variables|Default|GetcurrLevelStream))
        (EventDispatchers|UnbindEventfromOnLevelLoaded (Variables|Default|GetcurrLevelStream) (delegate Custom|OnLevelLoaded))
        (Variables|Default|SetCurrentLevel (Variables|Default|GetTargetLevel))
        (Default|CallOnNewState "NewEnumerator5")
        (Variables|Default|SetcurrLevelStream 0)))))

(event Custom|OnDeathTransEnd
  ;[1 1 1] Resets Rooms when player is destroyed
  (EventDispatchers|UnbindEventfromOnFadeComplete (Variables|Default|GetfadeWidget) (delegate Custom|OnDeathTransEnd))
  (Utilities|FlowControl|Delay 1.5)
  (Default|CallOnNewState "NewEnumerator10"))

(event EventPostLogin
  (params (NewPlayer :type Player%20Controller%20Object%20Reference))
  ;[1 1 1] On Login
  (bind _output_get (Variables|Default|SetP_Controller NewPlayer))
  (bind _asp_controller (Utilities|Casting|CastToP_Controller _output_get))
  (Default|OnInit _asp_controller)
  (CallFunction|Respawn))

(event EventBeginPlay
  (EventDispatchers|BindEventtoOnNewState (delegate Custom|NewState))
  (Default|CallOnNewState "NewEnumerator0"))

(fn ConstructionScript)

(fn InitGameMode
  (Variables|Default|SetCurrentGameState "NewEnumerator0")
  (bind _returnvalue (Game|SpawnActorfromClass "/Game/Blueprints/Managers/BP_SoundManager.BP_SoundManager_C" (Math|Transform|MakeTransform "0, 0, 0" "0, 0, 0" "1,1,1") "Undefined" 0 0))
  (Variables|Default|SetSound%20Manager _returnvalue)
  (bind _returnvalue_2 (UserInterface|CreateWidget "/Game/Blueprints/UI/Widget_ScreenFade.Widget_ScreenFade_C"))
  (bind _output_get (Variables|Default|SetfadeWidget _returnvalue_2))
  (UserInterface|Viewport|AddtoViewport _output_get 0)
  (Actor|GetAllActorsOfClass "/Game/Blueprints/MIsc/BP_PlayerSpawn.BP_PlayerSpawn_C")
  (CallFunction|CreateNewController)
  (CallFunction|UnloadAllLevels))

(fn CreateNewController
  (Class|GameplayStatics|RemovePlayer (Game|GetPlayerController 0) true)
  (Class|GameplayStatics|CreatePlayer -1))

(fn SetUpCharacter
  (Variables|Default|SetCurrentGameState "NewEnumerator5")
  (Utilities|IsValid (Variables|Default|GetP_Controller)
    (:Is%20Valid
      (bind _returnvalue (Game|SpawnActorfromClass "/Game/Blueprints/Pawn/BP_Char_Player.BP_Char_Player_C" (Math|Transform|MakeTransform "0, 0, 0" "0, 0, 0" "1,1,1") "AdjustIfPossibleButAlwaysSpawn" 0 0))
      (bind _output_get (Variables|Default|SetPlayerCharacter _returnvalue))
      (Pawn|Possess (Variables|Default|GetP_Controller) _output_get)
      (Class|IInitialisable|Init(Message) (Variables|Default|GetPlayerCharacter))
      (CallFunction|RespawnBinding)
      (Default|CallOnNewState "NewEnumerator13"))
    (:Is%20Not%20Valid
      (Development|PrintString "Controller Is null!!!!" true true "(R=1.000000,G=0.000000,B=0.002769,A=1.000000)"))))

(fn BeginLoadLevel
  (params (New%20Level :type E_Levels%20Enum :default "NewEnumerator0"))
  (switch Utilities|FlowControl|Switch|SwitchonE_Levels New%20Level
    (:NewEnumerator1
      (CallFunction|LoadLevel "Level1" "0, 0, 0" "0, 0, 0" true))))

(fn LoadLevel
  (params (LevelName :type String) (Location :type Vector) (Rotation :type Rotator) (bShouldBeVisible :type Boolean))
  (if (not (Class|LevelStreaming|IsLevelLoaded (Class|GameplayStatics|GetStreamingLevel (Utilities|String|StringToName LevelName))))
    (bind (_boutsuccess _returnvalue) (Class|LevelStreamingDynamic|LoadLevelInstance LevelName Location Rotation))
    (CallFunction|BindtoLevelLoaded _returnvalue)
    (if _boutsuccess
      (Variables|/Script/Engine.LevelStreaming|SetbShouldBeVisible _returnvalue bShouldBeVisible)
      (return _boutsuccess)
      (else
        (return _boutsuccess)))))

(fn BeginUnLoadLevel
  (params (New%20Level :type E_Levels%20Enum :default "NewEnumerator0"))
  (switch Utilities|FlowControl|Switch|SwitchonE_Levels New%20Level
    (:NewEnumerator1
      (CallFunction|OnUnLoadLevel "Level1-demoForWeek3Build"))))

(fn UnloadAllLevels
  (for _index (range 0 (Variables|Default|Getmax%20nLevels))
    (CallFunction|BeginUnLoadLevel (Utilities|Enum|ByteToEnumE_Levels (Math|Conversions|ToByte(Integer) _index))))
  (Default|CallOnAllLevelsUnloaded))

(fn SpawnPlayer
  (Variables|Default|SetCurrentGameState "NewEnumerator12")
  (Utilities|IsValid (Variables|Default|GetcurrentSpawnPoint)
    (:Is%20Valid
      (Default|SetCamLagSpeed (Variables|Default|GetPlayerCharacter) false 0.0)
      (bind _spawnpoint (Default|GetSpawnPoint (Variables|Default|GetcurrentSpawnPoint)))
      (Transformation|SetActorLocation (Variables|Default|GetPlayerCharacter) _spawnpoint false false)
      (Transformation|SetActorRotation (Variables|Default|GetPlayerCharacter) (Transformation|GetActorRotation (Variables|Default|GetcurrentSpawnPoint)))
      (Default|CallOnNewState "NewEnumerator4"))
    (:Is%20Not%20Valid
      (Development|PrintString "No Valid Spawn Point" true true "(R=1.000000,G=0.193575,B=0.000000,A=1.000000)"))))

(fn GetActiveSpawn
  (Variables|Default|SetCurrentGameState "NewEnumerator13")
  (bind _outactors (Actor|GetAllActorsOfClass "/Game/Blueprints/MIsc/BP_PlayerSpawn.BP_PlayerSpawn_C"))
  (bind _array_element (Utilities|Array|ForEachLoopwithBreak _outactors :!label _label)
    (:LoopBody
      (bind _parentlevel (Default|GetParentLevel _array_element))
      (if (== _parentlevel (Variables|Default|GetCurrentLevel))
        (Variables|Default|SetcurrentSpawnPoint _array_element)
        (goto _label Break)))
    (:Completed
      (Utilities|IsValid (Variables|Default|GetcurrentSpawnPoint)
        (:Is%20Valid
          (Default|CallOnNewState "NewEnumerator12")
          (return true))
        (:Is%20Not%20Valid
          (return false))))))

(fn LoadNextLevel
  (params (NextLevel :type E_Levels%20Enum :default "NewEnumerator1"))
  (Variables|Default|SetCurrentGameState "NewEnumerator14")
  (CallFunction|BeginLoadLevel NextLevel))

(fn EndTransition
  (Default|OnFadeOut (Variables|Default|GetfadeWidget)))

(fn GetLevelName
  (params (NextLevel :type E_Levels%20Enum :default "NewEnumerator1"))
  (switch Utilities|FlowControl|Switch|SwitchonE_Levels NextLevel
    (:NewEnumerator1
      (return "Level1-demoForWeek3Build"))))

(fn InitUI
  (bind _playercharacter (Variables|Default|GetPlayerCharacter))
  (Variables|Default|SetCurrentGameState "NewEnumerator15")
  (Default|ToggleHUD _playercharacter true)
  (Default|ToggleBuffSelectUI _playercharacter true)
  (CallFunction|NewState "NewEnumerator7"))

(fn DisablePlayerUI
  (Default|ToggleHUD (Variables|Default|GetPlayerCharacter) false)
  (Default|ToggleBuffSelectUI (Variables|Default|GetPlayerCharacter) false))

(fn RespawnPlayer
  (Variables|Default|SetCurrentGameState "NewEnumerator12")
  (Utilities|IsValid (Variables|Default|GetcurrentSpawnPoint)
    (:Is%20Valid
      (Default|SetCamLagSpeed (Variables|Default|GetPlayerCharacter) false 0.0)
      (bind _spawnpoint (Default|GetSpawnPoint (Variables|Default|GetcurrentSpawnPoint)))
      (Transformation|SetActorLocation (Variables|Default|GetPlayerCharacter) _spawnpoint false false)
      (Transformation|SetActorRotation (Variables|Default|GetPlayerCharacter) (Transformation|GetActorRotation (Variables|Default|GetcurrentSpawnPoint)))
      (Default|CallOnNewState "NewEnumerator11"))
    (:Is%20Not%20Valid
      (Development|PrintString "No Valid Spawn Point" true true "(R=1.000000,G=0.193575,B=0.000000,A=1.000000)"))))

(fn GetGameModeRef
  (return self))

(fn GetGameState
  (return (Variables|Default|GetCurrentGameState)))

(fn GetSoundManager
  (return (Variables|Default|GetSound%20Manager)))
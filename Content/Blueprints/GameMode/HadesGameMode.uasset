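; HadesGameMode is the game mode that spawns the player character and resets rooms when the player dies.
; BeginPlay caches enemy area managers, spawn triggers and a PlayerStart location, keeping the last start found.
; PostLogin stores the controller and calls Respawn, which after a short delay spawns BP_Char_Player, possesses it and rebinds its death event.
; On death, it respawns the player and sends IResetMessage to every cached manager and trigger.
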(event Custom|Respawn
  ;[1 1 1] Respawn
  (Utilities|FlowControl|Delay 1.0)
  (bind _returnvalue (Game|SpawnActorfromClass "/Game/Blueprints/Pawn/BP_Char_Player.BP_Char_Player_C" (Math|Conversions|ToTransform(Vector) (Variables|Default|GetRespawn%20Location)) "Undefined" 0 0)) ; Spawns a new character actor
  (Variables|Default|SetPawn _returnvalue)
  (Pawn|Possess (Variables|Default|GetP_Controller) _returnvalue) ; Posses
  (CallFunction|RespawnBinding) ; Binds again for new pawn
)

(event Custom|Respawn%20Binding
  ;[1 1 1] Resets Rooms when player is destroyed
  (EventDispatchers|BindEventtoPlayerDied (Variables|Default|GetPawn) (delegate Custom|Player%20Died)))

(event Custom|Player%20Died
  ;[1 1 1] Resets Rooms when player is destroyed
  (CallFunction|Respawn)
  (for _array_element (Variables|Default|GetManagers) ; Resets managers
    (Class|ITrigger|IReset(Message) _array_element))
  (for _array_element_2 (Variables|Default|GetSpawn%20Triggers) ; Resets Spawn Triggers
    (Class|ITrigger|IReset(Message) _array_element_2)))

(event EventPostLogin
  (params (NewPlayer :type Player%20Controller%20Object%20Reference))
  (Variables|Default|SetP_Controller NewPlayer)
  (CallFunction|Respawn))

(event EventBeginPlay
  (bind _outactors (Actor|GetAllActorsOfClass "/Game/Blueprints/Managers/BP_EnemyAreaManager.BP_EnemyAreaManager_C"))
  (Variables|Default|SetManagers _outactors)
  (bind _outactors_2 (Actor|GetAllActorsOfClass "/Script/Engine.PlayerStart"))
  (for _array_element _outactors_2
    (Variables|Default|SetRespawn%20Location (Transformation|GetActorLocation _array_element)))
  (bind _outactors_3 (Actor|GetAllActorsOfClass "/Game/Blueprints/Environment/BP_SpawnTrigger.BP_SpawnTrigger_C"))
  (Variables|Default|SetSpawn%20Triggers _outactors_3))

(fn ConstructionScript)
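; I_Pawn is a Blueprint Interface that defines a common set of calls for pawns, mostly combat-related.
; Getters expose the equipped weapon, team, mesh, melee attack data and hurt data, which covers hurt time and flash rate.
; Further calls set input buffer listening states, trigger the input buffer, and request a random point within a sphere.
; The functions are signatures only, with behaviour left to implementing classes.
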(fn IGetWeaponEquipped
  (return 0))

(fn IGetTeam
  (return "NewEnumerator0"))

(fn IGetMesh
  (return 0))

(fn ISetBufferListening
  (params (BufferStates :type EBufferStates%20Enum :default "NewEnumerator0")))

(fn ITriggerInputBuffer)

(fn IGetMeleeAttackData
  (return ""))

(fn IRandomPointinSphere
  (params (centre :type Vector) (radius :type Float%20%28single-precision%29))
  (return "0, 0, 0"))

(fn IGetHurtData
  (return 0.0 0.0))
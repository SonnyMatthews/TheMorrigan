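; Sound manager Blueprint that plays music and positional SFX and holds the game's volume levels.
; PlayMusic stores the track and joins RestartMusic's logic, which spawns a 2D sound and binds an event to its finish.
; Setters write music and SFX volumes to the VolumeLevels struct, applied only when sounds spawn.
; Master volume has a getter but is not applied to playback here.
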(event Custom|Restart%20Music
  (bind _returnvalue (Audio|SpawnSound2D (Variables|Default|GetCurrent%20Music%20Wave) (Utilities|Struct|BreakS_SoundValues (Variables|Default|GetVolumeLevels)) 1.0 0.0 0))
  (bind _output_get (Variables|Default|SetCurrent%20Music _returnvalue))
  (EventDispatchers|BindEventtoOnAudioFinished _output_get (EventDispatchers|CreateEvent :!event Custom|Restart%20Music)))

(event EventSetSFXVolume
  (params (SFX%20Volume :type Float%20%28single-precision%29))
  (Utilities|Struct|SetmembersinS_SoundValues (Variables|Default|GetVolumeLevels) SFX%20Volume))

(event EventSetMusicVolume
  (params (Music%20Volume :type Float%20%28single-precision%29))
  (Utilities|Struct|SetmembersinS_SoundValues (Variables|Default|GetVolumeLevels) Music%20Volume))

(event EventPlaySFXatLocation
  (params (Sound :type Sound%20Cue%20Object%20Reference) (Location :type Vector :default "0, 0, 0") (Attenuation :type Sound%20Attenuation%20Object%20Reference))
  (Audio|SpawnSoundatLocation Sound Location "0, 0, 0" (Utilities|Struct|BreakS_SoundValues (Variables|Default|GetVolumeLevels)) 1.0 0.0 0 0))

(event EventPlayMusic
  (params (Music :type Sound%20Cue%20Object%20Reference))
  (Variables|Default|SetCurrent%20Music%20Wave Music)
  (bind _returnvalue (Audio|SpawnSound2D (Variables|Default|GetCurrent%20Music%20Wave) (Utilities|Struct|BreakS_SoundValues (Variables|Default|GetVolumeLevels)) 1.0 0.0 0))
  (bind _output_get (Variables|Default|SetCurrent%20Music _returnvalue))
  (EventDispatchers|BindEventtoOnAudioFinished _output_get (EventDispatchers|CreateEvent :!event Custom|Restart%20Music)))

(event EventStopMusic
  (Audio|Components|Audio|Stop (Variables|Default|GetCurrent%20Music)))

(fn ConstructionScript)

(fn GetMaterVolume
  (return (Utilities|Struct|BreakS_SoundValues (Variables|Default|GetVolumeLevels))))

(fn GetMusicVolume
  (return (Utilities|Struct|BreakS_SoundValues (Variables|Default|GetVolumeLevels))))

(fn GetSFXVolume
  (return (Utilities|Struct|BreakS_SoundValues (Variables|Default|GetVolumeLevels))))

(fn GetSoundManagerReference
  (return self))
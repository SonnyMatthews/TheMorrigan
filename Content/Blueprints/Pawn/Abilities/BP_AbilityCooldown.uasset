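; Helper actor that runs the cooldown for one pawn ability, started through the ITriggerCooldown event.
; After a start delay, it caches the owner's HUD and starts a looping 0.01-second timer that counts down the cooldown length.
; Each tick sends the remaining time to the HUD's ability slots and prints it for debugging.
; At zero it notifies the owner through ICooldownFinishedMessage and destroys itself.
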(event Custom|Cooldown
  (Variables|Default|SetCount (- (Variables|Default|GetCount) 0.01))
  (Class|IHUD|IUpdateAbilitySlots(Message) (Variables|Default|GetHUD) "" (- (Variables|Default|GetCount) 0.01) (Variables|Default|GetTempAbilityToCooldown))
  (Development|PrintString (Utilities|String|ToString(Float) (- (Variables|Default|GetCount) 0.01)))
  (if (<= (Variables|Default|GetCount) 0.0)
    (Class|ICharacter|ICooldownFinished(Message) (Variables|Default|GetTempOwner) (Variables|Default|GetTempAbilityToCooldown))
    (Actor|DestroyActor)))

(event EventITriggerCooldown
  (params (Owner :type Actor%20Object%20Reference) (AbilityToCooldown :type EAbility%20Enum :default "NewEnumerator0") (CooldownLength :type Float%20%28single-precision%29) (TimeTillCooldownStart :type Float%20%28single-precision%29))
  (Variables|Default|SetTempOwner Owner)
  (Variables|Default|SetTempAbilityToCooldown AbilityToCooldown)
  (bind _output_get (Variables|Default|SetCooldownLength CooldownLength))
  (Variables|Default|SetCount _output_get)
  (Utilities|FlowControl|Delay TimeTillCooldownStart)
  (bind _hud (Class|ICharacter|GetHUD(Message) (Variables|Default|GetTempOwner)))
  (Variables|Default|SetHUD _hud)
  (bind _returnvalue (Utilities|Time|SetTimerbyEvent (delegate Custom|Cooldown) 0.01 true))
  (Variables|Default|SetCooldownTimer _returnvalue)
  (Development|PrintString "HERE?"))

(fn ConstructionScript)
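; Base actor for pawn abilities that activates once, runs a cooldown shown on the HUD, then destroys itself.
; ITriggerCooldown fetches the owner's HUD and calls ActivateAbility, a stub returning success and zero cooldown, destroying the actor if activation fails.
; On success, it waits the passed-in length, then a fast looping timer counts down the returned cooldown, updating the HUD ability slot until expiry.
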(event Custom|TimeDown
  (bind _output_get (Variables|Default|SetCount (- (Variables|Default|GetCount) 0.01)))
  (Class|IHUD|IUpdateAbilitySlots(Message) (Variables|Default|GetHUD) (Variables|Default|GetSlotName) _output_get "NewEnumerator0")
  (if (<= _output_get 0.0)
    (Actor|DestroyActor)))

(event EventITriggerCooldown
  (params (Owner :type Actor%20Object%20Reference) (AbilityToCooldown :type EAbility%20Enum :default "NewEnumerator5") (CooldownLength :type Float%20%28single-precision%29) (TimeTillCooldownStart :type Float%20%28single-precision%29))
  (Variables|Default|SetTimeTillStartCooldown CooldownLength)
  (bind _hud (Class|ICharacter|GetHUD(Message) Owner))
  (Variables|Default|SetHUD _hud)
  (bind (_activated_ _cooldown) (CallFunction|ActivateAbility Owner))
  (bind _output_get (Variables|Default|SetTimeTillActiveAgain _cooldown))
  (Variables|Default|SetCount _output_get)
  (if _activated_
    (Utilities|FlowControl|Delay (Variables|Default|GetTimeTillStartCooldown))
    (bind _returnvalue (Utilities|Time|SetTimerbyEvent (delegate Custom|TimeDown) 0.01 true))
    (Variables|Default|SetAbilityTimer _returnvalue)
    (else
      (Actor|DestroyActor))))

(fn ConstructionScript)

(fn ActivateAbility
  (params (Owner :type Actor%20Object%20Reference))
  (return true 0.0))
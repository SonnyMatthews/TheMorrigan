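; Base ability actor whose lifetime doubles as the ability's cooldown.
; TriggerAbility stores the timings and calls ActivateAbility, a stub returning true that presumably child abilities override, destroying the actor on failure.
; On success it waits out a delay, then a fast looping timer counts the cooldown down.
; The countdown prints each tick as debug output, then prints the class name and destroys the actor at zero.
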(event Custom|TimeDown
  (bind _output_get (Variables|Default|SetCount (- (Variables|Default|GetCount) 0.01)))
  (Development|PrintString (Utilities|String|ToString(Float) _output_get))
  (if (<= _output_get 0.0)
    (Development|PrintString (Utilities|GetClassDisplayName (Utilities|GetClass self)))
    (Actor|DestroyActor)))

(event EventTriggerAbility
  (params (Owner :type Actor%20Object%20Reference) (TimeTillStartCooldown :type Float%20%28single-precision%29) (Cooldown :type Float%20%28single-precision%29))
  (Variables|Default|SetTimeTillStartCooldown TimeTillStartCooldown)
  (bind _output_get (Variables|Default|SetTimeTillActiveAgain Cooldown))
  (Variables|Default|SetCount _output_get)
  (bind _activated_ (CallFunction|ActivateAbility Owner))
  (if _activated_
    (Utilities|FlowControl|Delay (Variables|Default|GetTimeTillStartCooldown))
    (bind _returnvalue (Utilities|Time|SetTimerbyEvent (delegate Custom|TimeDown) 0.01 true))
    (Variables|Default|SetAbilityTimer _returnvalue)
    (else
      (Actor|DestroyActor))))

(fn ConstructionScript)

(fn ActivateAbility
  (params (Owner :type Actor%20Object%20Reference))
  (return true))
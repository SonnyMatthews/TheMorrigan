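; BP_GroundPound is an area-of-effect ability that damages and knocks back enemies around its owner.
; On activation it pulls AOE stats from the Game Instance, then sphere-overlaps Pawns of class BP_BaseEnemy at the owner's location.
; Each hit enemy receives damage and knockback through DamageMessage, and the ability returns success with its cooldown to the caller.
; A debug sphere and damage printout run on every activation.
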(event EventBeginPlay)

(event Collision|EventActorBeginOverlap
  (params (OtherActor :type Actor%20Object%20Reference)))

(event EventTick
  (params (DeltaSeconds :type Float%20%28single-precision%29)))

(fn ConstructionScript
  (|CallParentFunction))

(fn ActivateAbility
  (params (Owner :type Actor%20Object%20Reference))
  (LocalVariables|SetTempOwner Owner)
  (bind _stats (Class|IInstance|GetPlayerStats(Message) (Game|GetGameInstance)))
  (bind _output_get (LocalVariables|SetTempStats (.aoe_stats _stats)))
  (Development|PrintString (Utilities|String|ToString(Float) (.aoe_damage _output_get)))
  (Rendering|Debug|DrawDebugSphere (Transformation|GetActorLocation (LocalVariables|GetTempOwner)) (Utilities|Struct|BreakS_AOEStats (LocalVariables|GetTempStats)) 12 "(R=1.000000,G=1.000000,B=1.000000,A=1.000000)" 5.0 2.0)
  (bind _outactors (Collision|SphereOverlapActors (Transformation|GetActorLocation (LocalVariables|GetTempOwner)) (Utilities|Struct|BreakS_AOEStats (LocalVariables|GetTempStats)) (Utilities|Array|MakeArray "ObjectTypeQuery3") "/Game/Blueprints/AI/Characters/BP_BaseEnemy.BP_BaseEnemy_C" (Utilities|Array|MakeArray (LocalVariables|GetTempOwner))))
  (for _array_element _outactors
    (Class|IDamageable|Damage(Message) _array_element (.AOE_Damage (Utilities|Struct|BreakS_AOEStats (LocalVariables|GetTempStats))) (.AOE_Knockback (Utilities|Struct|BreakS_AOEStats (LocalVariables|GetTempStats))) self))
  (return true (.AOE_Cooldown (Utilities|Struct|BreakS_AOEStats (LocalVariables|GetTempStats)))))
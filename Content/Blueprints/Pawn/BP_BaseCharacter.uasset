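; Base character Blueprint that provides shared damage, knockback, hurt feedback and weapon attachment for pawns.
; Damage launches the character away from the hit location, deducts health, then calls an empty Death stub or updates the health UI.
; A separate OnHurt event uses timers to flash the mesh between hurt and default materials.
; Helpers play hit effects and expose combat data through interface getters, while SetStats has its data-table logic disconnected.
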(event Custom|OnHurt
  ;[1 1 1] Hurt flash
  (Variables|States|SetisHurt true)
  (Utilities|Time|SetTimerbyEvent (delegate Custom|FinishHurt) (Variables|Timers|GethurtTime))
  (CallFunction|Flashon)
  (bind _returnvalue (Utilities|Time|SetTimerbyEvent (delegate Custom|ToggleFlash) (Variables|Timers|GetFlashRate) true))
  (Variables|Timers|SetFlashTimerHandle _returnvalue))

(event Custom|FinishHurt
  ;[1 1 1] Hurt flash
  (Utilities|Time|PauseTimerbyHandle (Variables|Timers|GetFlashTimerHandle))
  (CallFunction|FlashOff)
  (Variables|States|SetisHurt false))

(event Custom|ToggleFlash
  ;[1 1 1] Hurt flash
  (if (Variables|States|GetIsFlashOn)
    (CallFunction|FlashOff)
    (else
      (CallFunction|Flashon))))

(event EventBeginPlay
  (bind _soundmanager (Class|IMorriganGameMode|GetSoundManager(Message) (Game|GetGameMode)))
  (Variables|Default|SetSoundManager _soundmanager))

(event EventDamage
  (params (Damage :type Float%20%28single-precision%29) (KnockBack :type Float%20%28single-precision%29) (InterfacingActor :type Actor%20Object%20Reference) (ActorLocation :type Vector :default "0, 0, 0"))
  ;[1 1 1] Damage
  (CallFunction|AddImpulseinDirection ActorLocation KnockBack)
  (bind _isdead_ (CallFunction|DeductHealth Damage))
  (if _isdead_
    (CallFunction|Death)
    (else
      (CallFunction|UpdateHealth))))

(fn ConstructionScript
  (Transformation|AttachComponentToComponent (Variables|Default|GetWeapon) (Variables|Character|GetMesh) "Socket_Weapon" "KeepRelative" "KeepRelative" "KeepWorld" true)
  (Variables|Default|SetdefaultMaterial (Rendering|Material|GetMaterial (Variables|Character|GetMesh) 0)))

(fn SetStats
  (params (RowName :type Name) (DataTable :type Data%20Table%20Object%20Reference)))

(fn DeductHealth
  (params (HealthToDeduct :type Float%20%28single-precision%29))
  (bind _output_get (Variables|Stats|SetCurrentHealth (- (Variables|Stats|GetCurrentHealth) HealthToDeduct)))
  (return (<= _output_get 0.0)))

(fn Death)

(fn UpdateHealth
  (Default|CallUpdateHealthUI 0.0))

(fn AddImpulseinDirection
  (params (StartLocationOfImpulse :type Vector) (StrengthOfImpulse :type Float%20%28single-precision%29))
  (LocalVariables|SetTempStartLocationOfImpulse StartLocationOfImpulse)
  (bind _output_get (LocalVariables|SetTempImpulseStrength StrengthOfImpulse))
  (if (not (== _output_get 0.0))
    (AI|Navigation|StopMovement (Pawn|GetController))
    (Collision|LineTraceByChannel (Transformation|GetActorLocation) (+ (LocalVariables|GetTempStartLocationOfImpulse) (* (Math|Vector|GetUnitDirection(Vector) (LocalVariables|GetTempStartLocationOfImpulse) (Transformation|GetActorLocation)) (LocalVariables|GetTempImpulseStrength))) "TraceTypeQuery1" false 0 "None" true "(R=1.000000,G=0.000000,B=0.000000,A=1.000000)" "(R=0.000000,G=1.000000,B=0.000000,A=1.000000)" 1e+01)
    (Character|LaunchCharacter (Math|Vector|MakeVector (.X (Math|Vector|BreakVector (* (Math|Vector|GetUnitDirection(Vector) (LocalVariables|GetTempStartLocationOfImpulse) (Transformation|GetActorLocation)) (LocalVariables|GetTempImpulseStrength)))) (.Y (Math|Vector|BreakVector (* (Math|Vector|GetUnitDirection(Vector) (LocalVariables|GetTempStartLocationOfImpulse) (Transformation|GetActorLocation)) (LocalVariables|GetTempImpulseStrength)))) 0.0) true false)))

(fn Flashon
  (bind _returnvalue (Rendering|Material|CreateDynamicMaterialInstance (Variables|Character|GetMesh) 0 (Variables|Default|GethurtMat) "None" :!class /Script/Engine.PrimitiveComponent))
  (Rendering|Material|SetVectorParameterValue _returnvalue "FlashCol" (Variables|Default|GetflashColour) :!class /Script/Engine.MaterialInstanceDynamic)
  (Variables|States|SetIsFlashOn true))

(fn FlashOff
  (bind _returnvalue (Rendering|Material|CreateDynamicMaterialInstance (Variables|Character|GetMesh) 0 (Variables|Default|GetdefaultMaterial) "None" :!class /Script/Engine.PrimitiveComponent))
  (Rendering|Material|SetVectorParameterValue _returnvalue "FlashCol" (Variables|Default|GetflashColour) :!class /Script/Engine.MaterialInstanceDynamic)
  (Variables|States|SetIsFlashOn false))

(fn GetRandPointinSphere
  (params (Centre :type Vector) (Radius :type Float%20%28single-precision%29))
  (return (+ Centre (* (Math|Random|RandomUnitVector) (Math|Random|RandomFloatinRange 0.0 Radius)))))

(fn HitSoundEffect
  (Class|ISound|PlaySFXatLocation(Message) (Variables|Default|GetSoundManager) (Variables|Default|GetDamageSoundEffect) (Transformation|GetActorLocation)))

(fn SpawnParticleEffect
  (params (LocationOfHit :type Vector) (EmitterTemplate :type Particle%20System%20Object%20Reference))
  (Effects|SpawnEmitterAttached EmitterTemplate (Variables|Character|GetMesh) "None" "0, 0, 0" "0, 0, 0" "1.000000,1.000000,1.000000" "SnapToTarget"))

(fn IGetHurtData
  (return (Variables|Timers|GethurtTime) (Variables|Timers|GetFlashRate)))

(fn IGetMeleeAttackData
  (return (Variables|Stats|GetMeleeAttackAnimationData)))

(fn IGetMesh
  (return 0))

(fn IGetTeam
  (return "NewEnumerator0"))

(fn IGetWeaponEquipped
  (return (Variables|/Script/Engine.ChildActorComponent|GetChildActor (Variables|Default|GetWeapon))))

(fn IRandomPointinSphere
  (params (centre :type Vector :default "0, 0, 0") (radius :type Float%20%28single-precision%29))
  (bind _randpoint (CallFunction|GetRandPointinSphere centre radius))
  (return _randpoint))
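; Player character for an action game, with melee, thrust, evade dash, projectile and AOE attacks aimed by mouse or gamepad.
; Stats, montages and curves load from DT_PlayerStats.
; A CurrentState enum gates melee, thrust and evade and queues the latest blocked input, while retimed timelines drive swept lunges and dashes.
; DoOnce nodes with delays handle cooldowns; starting-buff and permanent-upgrade logic is mostly stubbed or disconnected.
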(event OnComponentBeginOverlap(CapsuleComponent)
  (params (OverlappedComponent :type Primitive%20Component%20Object%20Reference) (OtherActor :type Actor%20Object%20Reference) (OtherComp :type Primitive%20Component%20Object%20Reference) (OtherBodyIndex :type Integer) (bFromSweep :type Boolean) (SweepResult :type Hit%20Result%20Structure%20%28by%20ref%29))
  ;[1 1 1] Overlap Damage
  (if (Utilities|Enum|Equal(Enum) (Variables|Default|GetCurrentState) "NewEnumerator1")
    (Class|IDamageable|Damage(Message) OtherActor 2e+01 0.0 self)
    (Audio|PlaySound2D "/Engine/EditorSounds/Notifications/CompileFailed.CompileFailed" 1.0 1.0 0.0 0 0)))

(event Custom|ResetEvade
  ;[1 1 1] Evade
  (Utilities|FlowControl|DoOnce false) ; enters at Reset
)

(event Custom|AOE_Reset
  (bind _aoestats (Variables|Default|GetAOEStats))
  (bind (_aoe_damage _aoe_cooldown _aoe_knockback) (Utilities|Struct|BreakS_AOEStats _aoestats))
  ;[1 1 1] AOE
  (Utilities|FlowControl|DoOnce false) ; enters at Reset
)

(event Custom|AttackAnimation
  ;[1 1 1] Attack Animation
  (Audio|PlaySound2D "/Engine/VREditor/Sounds/UI/Click_on_Button.Click_on_Button" 1.0 (Utilities|Select :Index (Variables|Default|GetCurrentState) :NewEnumerator3 0.0 :NewEnumerator0 1.0 :NewEnumerator2 1.0 :NewEnumerator4 0.5 :NewEnumerator1 0.0) 0.0 0 0)
  (Variables|Default|SetStartLocation (Transformation|GetActorLocation))
  (bind _notifyname (Animation|Montage|PlayMontage (Variables|Character|GetMesh) (.Montage (CallFunction|GetAttackAnimationData (Variables|Default|GetCurrentState))) (.Speed (CallFunction|GetAttackAnimationData (Variables|Default|GetCurrentState))))
    (:OnCompleted
      (if (Variables|Default|GetQueuedInput?)
        (CallFunction|InputQueueActionTrigger)))
    (:OnNotifyBegin
      (Utilities|IsMoveForwardNotify? _notifyname)
      (CallFunction|SetTimelineProperties (Variables|Default|GetAttackMovement) (.Curve (CallFunction|GetAttackMovementData (Variables|Default|GetCurrentState))))
      (Variables|Default|SetTargetLocation (CallFunction|GetForwardMomentum (Variables|Default|GetStartLocation) (.Distance (CallFunction|GetAttackMovementData (Variables|Default|GetCurrentState)))))
      (bind _alpha (Timeline|AttackMovement PlayFromStart)
        (:Update
          (Transformation|SetActorLocation (Math|Vector|Lerp(Vector) (Variables|Default|GetStartLocation) (Variables|Default|GetTargetLocation) _alpha) true false))
        (:Finished
          (switch Utilities|FlowControl|Switch|SwitchonEInputState (Variables|Default|GetCurrentState)
            (:NewEnumerator0
              (Utilities|FlowControl|Delay (.MeleeCooldown (Utilities|Struct|BreakS_LightMeleeStats (Variables|Default|GetMeleeStats))) :!label _label)
              (Variables|Default|SetCurrentState "NewEnumerator3"))
            (:NewEnumerator2
              (goto _label))
            (:NewEnumerator4
              (Variables|Default|SetCurrentState "NewEnumerator3")
              (Utilities|FlowControl|Delay (Utilities|Struct|BreakS_ThrustAttackStats (Variables|Default|GetThrustStats)))
              (CallFunction|ResetThrust))))))))

(event Custom|ResetProjectile
  (bind _projectilestats (Variables|Default|GetProjectileStats))
  (bind _projectilestats_2 (Variables|Default|GetProjectileStats))
  (bind (_projectiledamage _projectilestartspeed _projectilemaxspeed _gravity _lifespan _maxenemycanhit) (Utilities|Struct|BreakS_ProjectileStats _projectilestats))
  (bind (_projectiledamage_2 _projectilestartspeed_2 _projectilemaxspeed_2 _gravity_2 _lifespan_2 _maxenemycanhit_2) (Utilities|Struct|BreakS_ProjectileStats _projectilestats_2))
  ;[1 1 1] Projectile Throw
  (Utilities|FlowControl|Sequence
    (:then_0
      (Utilities|FlowControl|DoOnce false) ; enters at Reset
    )
    (:then_1
      (Utilities|FlowControl|DoOnce false) ; enters at Reset
    )))

(event Custom|RemoveBuff
  ;[1 1 1] Remove buff after death
)

(event Custom|ChooseStartBuff
  (params (Buff :type Enum_Pickup%20Enum :default "NewEnumerator0"))
  ;[1 1 1] Set starting buff
)

(event Custom|ResetThrust
  ;[1 1 1] Thrust Input
  (Utilities|FlowControl|DoOnce false) ; enters at Reset
)

(event EventTick
  (params (DeltaSeconds :type Float%20%28single-precision%29))
  (bind _returnvalue (Game|GetPlayerController 0))
  (bind (_worldlocation _worlddirection) (Game|Player|ConvertMouseLocationToWorldSpace _returnvalue))
  ;[1 1 1] Set Mouse Loc and Projectile Direction
  (bind _outhit (CallFunction|GetMouseLocationinWorld _worldlocation _worlddirection))
  (bind _output_get (Variables|Default|SetMouseLocTick (.Location (Collision|BreakHitResult _outhit))))
  (Transformation|SetWorldRotation (Variables|Default|GetProjectileAimMouse) (Math|Rotator|MakeRotator (.roll (Math|Rotator|FindLookatRotation (Transformation|GetActorLocation) _output_get)) 0.0 (.yaw (Math|Rotator|FindLookatRotation (Transformation|GetActorLocation) _output_get))) false false))

(event EventIProjectileThrowMouse
  (bind _projectilestats (Variables|Default|GetProjectileStats))
  (bind (_projectiledamage _projectilestartspeed _projectilemaxspeed _gravity _lifespan _maxenemycanhit) (Utilities|Struct|BreakS_ProjectileStats _projectilestats))
  ;[1 1 1] Projectile Throw
  (Utilities|FlowControl|DoOnce false
    (:Completed
      (Utilities|FlowControl|Delay (Utilities|Struct|BreakS_ProjectileStats (Variables|Default|GetProjectileStats)))
      (Game|SpawnActorfromClass "/Game/Blueprints/Pawn/BP_ProjectileForPlayer.BP_ProjectileForPlayer_C" (Transformation|GetWorldTransform (Variables|Default|GetProjectileAimMouse)) "Undefined" 0 _projectiledamage _projectilestartspeed _projectilemaxspeed _gravity _lifespan _maxenemycanhit "0.000000,0.000000,0.000000" self)
      (Utilities|FlowControl|Delay (Utilities|Struct|BreakS_ProjectileStats (Variables|Default|GetProjectileStats)))
      (CallFunction|ResetProjectile))))

(event EventIProjectileThrowController
  (bind _projectilestats (Variables|Default|GetProjectileStats))
  (bind (_projectiledamage _projectilestartspeed _projectilemaxspeed _gravity _lifespan _maxenemycanhit) (Utilities|Struct|BreakS_ProjectileStats _projectilestats))
  ;[1 1 1] Projectile Throw
  (Utilities|FlowControl|DoOnce false
    (:Completed
      (CallFunction|SetPlayerRotationfromXY)
      (Utilities|FlowControl|Delay (Utilities|Struct|BreakS_ProjectileStats (Variables|Default|GetProjectileStats)))
      (Game|SpawnActorfromClass "/Game/Blueprints/Pawn/BP_ProjectileForPlayer.BP_ProjectileForPlayer_C" (Transformation|GetWorldTransform (Variables|Default|GetControllerRotation)) "Undefined" 0 _projectiledamage _projectilestartspeed _projectilemaxspeed _gravity _lifespan _maxenemycanhit "0.000000,0.000000,0.000000" self)
      (Utilities|FlowControl|Delay (Utilities|Struct|BreakS_ProjectileStats (Variables|Default|GetProjectileStats)))
      (CallFunction|ResetProjectile))))

(event EventBeginPlay
  (bind _returnvalue (Game|GetPlayerController 0))
  ;[1 1 1] Init
  (|CallParentFunction)
  (CallFunction|FetchDataforPawn)
  (CallFunction|SetTimelineProperties (Variables|Default|GetAttackMovement) (.MeleeAttackForwardCurve (Utilities|Struct|BreakS_LightMeleeStats (Variables|Default|GetMeleeStats))))
  (CallFunction|SetTimelineProperties (Variables|Default|GetEvadeMovement) (Utilities|Struct|BreakS_DashStats (Variables|Default|GetDashStats)))
  (bind _returnvalue_2 (UserInterface|CreateWidget "/Game/Blueprints/UI/Widget_BasicHUD.Widget_BasicHUD_C"))
  (UserInterface|Viewport|AddtoViewport _returnvalue_2 0)
  (Variables|Default|SetRespawnLocation (Transformation|GetActorLocation))
  ;[1 1 1] Start buff pick interface, to be moved
  (bind _returnvalue_3 (UserInterface|CreateWidget "/Game/Blueprints/UI/Widget_StartingBuff.Widget_StartingBuff_C" _returnvalue))
  (Input|SetInputModeUIOnly _returnvalue _returnvalue_3 "DoNotLock")
  (bind _output_get (Variables|Default|SetStartBuffWidgetRef _returnvalue_3))
  (UserInterface|Viewport|AddtoViewport _output_get 0))

(event EventIThrustAttack
  (params (InputMethod :type EInputMethod%20Enum :default "NewEnumerator0"))
  ;[1 1 1] Thrust Input
  (Variables|Default|SetInputMethod InputMethod)
  (Utilities|FlowControl|DoOnce false
    (:Completed
      (Utilities|IsthePlayerNotPerformingAnAction?
        (:Yes
          (Variables|Default|SetQueuedInput? true)
          (Variables|Default|SetQueuedInputState "NewEnumerator4")
          (CallFunction|ResetThrust))
        (:No
          (Variables|Default|SetCurrentState "NewEnumerator4")
          (Variables|Default|SetQueuedInput? false)
          (CallFunction|SetPlayerRotationfromInput (Variables|Default|GetInputMethod))
          (CallFunction|AttackAnimation))))))

(event EventIAttack
  (params (InputMethod :type EInputMethod%20Enum :default "NewEnumerator0"))
  ;[1 1 1] Attack
  (Variables|Default|SetInputMethod InputMethod)
  (Utilities|IsthePlayerNotPerformingAnAction?
    (:Yes
      (Variables|Default|SetQueuedInput? true)
      (Variables|Default|SetQueuedInputState "NewEnumerator0"))
    (:No
      (Variables|Default|SetCurrentState "NewEnumerator0")
      (Variables|Default|SetQueuedInput? false)
      (CallFunction|SetPlayerRotationfromInput (Variables|Default|GetInputMethod))
      (CallFunction|AttackAnimation))))

(event EventIUpDown
  (params (Axis :type Float%20%28single-precision%29))
  ;[1 1 1] Move Character
  (Variables|Default|SetY_Input Axis)
  (Class|PawnMovementComponent|AddInputVector (Variables|Character|GetCharacterMovement) (Math|Vector|MakeVector (Variables|Default|GetX_Input) (Variables|Default|GetY_Input) 0.0) false))

(event EventILeftRight
  (params (Axis :type Float%20%28single-precision%29))
  ;[1 1 1] Move Character
  (Variables|Default|SetX_Input Axis)
  (Class|PawnMovementComponent|AddInputVector (Variables|Character|GetCharacterMovement) (Math|Vector|MakeVector (Variables|Default|GetX_Input) (Variables|Default|GetY_Input) 0.0) false))

(event EventIEvade
  ;[1 1 1] Evade
  (Utilities|IsthePlayerNotPerformingAnAction?
    (:Yes
      (Variables|Default|SetQueuedInput? true)
      (Variables|Default|SetQueuedInputState "NewEnumerator1"))
    (:No
      (Utilities|FlowControl|DoOnce false
        (:Completed
          (Variables|Default|SetCurrentState "NewEnumerator1")
          (Variables|Default|SetQueuedInput? false)
          (CallFunction|SetPlayerRotationfromXY)
          (Audio|PlaySound2D "/Game/SuperGrid/TutorialLevel/SoundEffects/Cue_Jump.Cue_Jump" 1.0 1.0 0.0 0 0)
          (bind _output_get (Variables|Default|SetStartLocation (Transformation|GetActorLocation)))
          (Variables|Default|SetTargetLocation (CallFunction|GetForwardMomentum _output_get (Utilities|Struct|BreakS_DashStats (Variables|Default|GetDashStats))))
          (Collision|SetCollisionResponsetoChannel (Variables|Default|GetCapsuleComponent) "ECC_Pawn" "ECR_Overlap")
          (bind _alpha (Timeline|EvadeMovement PlayFromStart)
            (:Update
              (Transformation|SetActorLocation (Math|Vector|Lerp(Vector) (Variables|Default|GetStartLocation) (Variables|Default|GetTargetLocation) _alpha) true false))
            (:Finished
              (Variables|Default|SetCurrentState "NewEnumerator3")
              (if (Variables|Default|GetQueuedInput?)
                (CallFunction|InputQueueActionTrigger))
              (Collision|SetCollisionResponsetoChannel (Variables|Default|GetCapsuleComponent) "ECC_Pawn" "ECR_Block")
              (Utilities|FlowControl|Delay (Utilities|Struct|BreakS_DashStats (Variables|Default|GetDashStats)))
              (CallFunction|ResetEvade))))))))

(event EventIInteract
  ;[1 1 1] Interact with object
)

(event EventIAttackMouse)

(event EventIAOEAttack
  (bind _aoestats (Variables|Default|GetAOEStats))
  (bind (_aoe_damage _aoe_cooldown _aoe_knockback) (Utilities|Struct|BreakS_AOEStats _aoestats))
  ;[1 1 1] AOE
  (Utilities|FlowControl|DoOnce false
    (:Completed
      (Utilities|FlowControl|Delay (Utilities|Struct|BreakS_AOEStats (Variables|Default|GetAOEStats)))
      (Audio|PlaySound2D "/Game/SuperGrid/TutorialLevel/SoundEffects/Cue_Portals.Cue_Portals" 1.0 1.0 0.0 0 0)
      (Rendering|Debug|DrawDebugSphere (Transformation|GetActorLocation) (Utilities|Struct|BreakS_AOEStats (Variables|Default|GetAOEStats)) 12 "(R=1.000000,G=1.000000,B=1.000000,A=1.000000)" 5.0 2.0)
      (bind _outactors (Collision|SphereOverlapActors (Transformation|GetActorLocation) (Utilities|Struct|BreakS_AOEStats (Variables|Default|GetAOEStats)) (Utilities|Array|MakeArray "ObjectTypeQuery3") "/Game/Blueprints/AI/Characters/BP_BaseEnemy.BP_BaseEnemy_C" (Utilities|Array|MakeArray self)))
      (for _array_element _outactors
        (Class|IDamageable|Damage(Message) _array_element _aoe_damage _aoe_knockback self)
        (Utilities|FlowControl|Delay _aoe_cooldown)
        (CallFunction|AOEReset))
      (Utilities|FlowControl|Delay (.AOE_Cooldown (Utilities|Struct|BreakS_AOEStats (Variables|Default|GetAOEStats))))
      (CallFunction|AOEReset))))

(fn ConstructionScript)

(fn SetTimelineProperties
  (params (Timeline :type Timeline%20Component%20Object%20Reference) (NewFloatCurve :type Curve%20Float%20Object%20Reference))
  (Class|TimelineComponent|SetFloatCurve Timeline NewFloatCurve "Alpha")
  (Components|Timeline|SetTimelineLength Timeline (.MaxTime (Math|Curves|GetTimeRange NewFloatCurve))))

(fn ChangeMeleeDamage
  (params (Change :type Float%20%28single-precision%29))
  (Utilities|Struct|SetmembersinS_PawnStats (Variables|Default|GetPlayerStats)))

(fn ChangeMeleeSpeed
  (params (Change :type Float%20%28single-precision%29))
  (Utilities|Struct|SetmembersinS_PawnStats (Variables|Default|GetPlayerStats)))

(fn ChangeSpellDamage
  (params (Change :type Float%20%28single-precision%29))
  (Utilities|Struct|SetmembersinS_PawnStats (Variables|Default|GetPlayerStats)))

(fn ChangeAOEDamage
  (params (Change :type Float%20%28single-precision%29))
  (Utilities|Struct|SetmembersinS_PawnStats (Variables|Default|GetPlayerStats)))

(fn ChangeStunningAttack
  (params (Change :type Float%20%28single-precision%29))
  (if (>= Change 1.0)
    _))

(fn PermanentUpgrade
  (params (Pickup :type S%20Upgrades%20Structure))
  (bind (_stat _potencystrength) (Utilities|Struct|BreakS_Upgrades Pickup))
  ;[1 1 1] Takes Pickup Information and switches to buff different stat based on type
  (LocalVariables|SetLocalPotency _potencystrength)
  (switch string _stat
    (:MeleeDamage
      (PermanentStatChange|ChangeMeleeDamage (LocalVariables|GetLocalPotency)))
    (:AttackSpeed
      (PermanentStatChange|ChangeMeleeSpeed (LocalVariables|GetLocalPotency)))
    (:StunningAttackBuff
      (PermanentStatChange|ChangeStunningAttack (LocalVariables|GetLocalPotency)))
    (:AOEDamage
      (PermanentStatChange|ChangeAOEDamage (LocalVariables|GetLocalPotency)))
    (:SpellDamageBuff
      (PermanentStatChange|ChangeSpellDamage (LocalVariables|GetLocalPotency)))))

(fn DamageOverTime
  (Development|PrintString "Dot Event"))

(fn GetMouseLocationinWorld
  (params (Location :type Vector) (Direction :type Vector))
  (bind _outhit (Collision|LineTraceByChannel Location (+ Location (* (* Direction (/ (.Z (Math|Vector|BreakVector Location)) (.Z (Math|Vector|BreakVector Direction)))) -2.0)) "TraceTypeQuery1" false 0 "None"))
  (return _outhit))

(fn GetLookatRotationfromCharacter
  (params (Target :type Vector%20%28by%20ref%29))
  (return (.Yaw (Math|Rotator|BreakRotator (Math|Rotator|FindLookatRotation (Transformation|GetActorLocation) Target)))))

(fn IGetWeaponEquipped
  (return (Variables|/Script/Engine.ChildActorComponent|GetChildActor (Variables|Default|GetWeapon))))

(fn IGetTeam
  (return (Variables|Default|GetETeam)))

(fn IGetMesh
  (return 0))

(fn GetForwardMomentum
  (params (Start :type Vector) (Distance :type Float%20%28single-precision%29))
  (return (+ Start (* (Math|Vector|GetForwardVector (Variables|Default|GetControllerRotation)) Distance))))

(fn InputQueueActionTrigger
  (switch Utilities|FlowControl|Switch|SwitchonEInputState (Variables|Default|GetQueuedInputState)
    (:NewEnumerator0
      (CallFunction|IAttack (Variables|Default|GetInputMethod)))
    (:NewEnumerator4
      (CallFunction|IThrustAttack (Variables|Default|GetInputMethod)))
    (:NewEnumerator1
      (CallFunction|IEvade))))

(fn SetPlayerRotationfromXY
  (bind _x_input (Variables|Default|GetX_Input))
  (bind _y_input (Variables|Default|GetY_Input))
  (Utilities|IsThereNoLeftStickInput? _x_input _y_input
    (:Yes
      (Transformation|SetActorRotation (Math|Conversions|RotationFromXVector (Math|Vector|MakeVector _x_input _y_input 0.0)))
      (Development|PrintString "HERE"))))

(fn SetPlayerRotationfromMouse
  (bind _returnvalue (Game|GetPlayerController 0))
  (bind (_worldlocation _worlddirection) (Game|Player|ConvertMouseLocationToWorldSpace _returnvalue))
  (bind _outhit (CallFunction|GetMouseLocationinWorld _worldlocation _worlddirection))
  (Transformation|SetActorRotation (Math|Rotator|MakeRotator 0.0 0.0 (CallFunction|GetLookatRotationfromCharacter (.Location (Collision|BreakHitResult _outhit)))))
  (CallFunction|AttackAnimation))

(fn UpdateHealth
  (|CallParentFunction))

(fn FetchDataforPawn
  (bind _charactermovement (Variables|Character|GetCharacterMovement))
  (bind _returnvalue (Utilities|GetDataTableRow "/Game/Blueprints/Data/DT_PlayerStats.DT_PlayerStats" "Iter1")
    (:then
      (Variables|Default|SetHealthAndMovementStats (.HealthAndMovement_Stats (Utilities|Struct|BreakS_PawnStats _returnvalue)))
      (Variables|Default|SetMeleeStats (.Melee_Stats (Utilities|Struct|BreakS_PawnStats _returnvalue)))
      (Variables|Default|SetAOEStats (.AOE_Stats (Utilities|Struct|BreakS_PawnStats _returnvalue)))
      (Variables|Default|SetProjectileStats (.Projectile_Stats (Utilities|Struct|BreakS_PawnStats _returnvalue)))
      (Variables|Default|SetDashStats (.Dash_Stats (Utilities|Struct|BreakS_PawnStats _returnvalue)))
      (Variables|Default|SetThrustStats (.Thrust_Stats (Utilities|Struct|BreakS_PawnStats _returnvalue)))
      (Variables|Default|SetCurrentHealth (.MaxHealth (Utilities|Struct|BreakS_HealthAndMovementStats (Variables|Default|GetHealthAndMovementStats))))
      (Variables|/Script/Engine.CharacterMovementComponent|SetMaxWalkSpeed _charactermovement (.MovementSpeed (Utilities|Struct|BreakS_HealthAndMovementStats (Variables|Default|GetHealthAndMovementStats))))
      (Variables|/Script/Engine.CharacterMovementComponent|SetMaxAcceleration _charactermovement (.MovementAcceleration (Utilities|Struct|BreakS_HealthAndMovementStats (Variables|Default|GetHealthAndMovementStats))))
      (Variables|/Script/Engine.CharacterMovementComponent|SetRotationRate (Variables|Character|GetCharacterMovement) (.RotationRate (Utilities|Struct|BreakS_HealthAndMovementStats (Variables|Default|GetHealthAndMovementStats)))))))

(fn GetAttackMovementData
  (params (CurrentState :type EInputState%20Enum :default "NewEnumerator3"))
  (bind _meleestats (Variables|Default|GetMeleeStats))
  (bind _meleestats_2 (Variables|Default|GetMeleeStats))
  (bind _meleeattackforwarddistance (Utilities|Struct|BreakS_LightMeleeStats _meleestats))
  (bind _meleeattackforwardcurve (Utilities|Struct|BreakS_LightMeleeStats _meleestats_2))
  (return (Utilities|Select :Index CurrentState :NewEnumerator3 0 :NewEnumerator0 _meleeattackforwardcurve :NewEnumerator2 _meleeattackforwardcurve :NewEnumerator4 (Utilities|Struct|BreakS_ThrustAttackStats (Variables|Default|GetThrustStats)) :NewEnumerator1 0) (Utilities|Select :Index CurrentState :NewEnumerator3 0.0 :NewEnumerator0 _meleeattackforwarddistance :NewEnumerator2 _meleeattackforwarddistance :NewEnumerator4 (Utilities|Struct|BreakS_ThrustAttackStats (Variables|Default|GetThrustStats)) :NewEnumerator1 0.0)))

(fn GetAttackAnimationData
  (params (Index :type EInputState%20Enum :default "NewEnumerator3"))
  (bind _meleestats (Variables|Default|GetMeleeStats))
  (bind _meleestats_2 (Variables|Default|GetMeleeStats))
  (bind _meleeanimmontage (Utilities|Struct|BreakS_LightMeleeStats _meleestats))
  (bind _meleeattackspeed (Utilities|Struct|BreakS_LightMeleeStats _meleestats_2))
  (return (Utilities|Select :Index Index :NewEnumerator3 0 :NewEnumerator0 _meleeanimmontage :NewEnumerator2 _meleeanimmontage :NewEnumerator4 (Utilities|Struct|BreakS_ThrustAttackStats (Variables|Default|GetThrustStats)) :NewEnumerator1 0) (Utilities|Select :Index Index :NewEnumerator3 0.0 :NewEnumerator0 _meleeattackspeed :NewEnumerator2 _meleeattackspeed :NewEnumerator4 (Utilities|Struct|BreakS_ThrustAttackStats (Variables|Default|GetThrustStats)) :NewEnumerator1 0.0)))

(fn Death
  (|CallParentFunction)
  (Default|CallPlayerDied))

(fn SetInputMethod
  (params (Key :type Key%20Structure%20%28by%20ref%29))
  (Variables|Default|SetInputMethod (select (Class|KismetInputLibrary|KeyIsGamepadKey Key) "NewEnumerator0" "NewEnumerator1")))

(fn SetPlayerRotationfromInput
  (params (InputMethod :type EInputMethod%20Enum :default "NewEnumerator0"))
  (switch Utilities|FlowControl|Switch|SwitchonEInputMethod InputMethod
    (:NewEnumerator0
      (CallFunction|SetPlayerRotationfromXY))
    (:NewEnumerator1
      (CallFunction|SetPlayerRotationfromMouse))))

(fn InputBufferingTrigger)
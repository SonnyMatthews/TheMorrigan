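; Player projectile actor that damages actors it overlaps, other than its instigator.
; The construction script applies lifespan, gravity, launch and max speed, and mesh scale from variables to the actor, ProjectileMovement and mesh.
; Each sphere overlap sends a DamageMessage with the damage amount and projectile location, then destroys the projectile once the hit count reaches its maximum, allowing it to pierce several targets.
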(event OnComponentBeginOverlap(Sphere)
  (params (OverlappedComponent :type Primitive%20Component%20Object%20Reference) (OtherActor :type Actor%20Object%20Reference) (OtherComp :type Primitive%20Component%20Object%20Reference) (OtherBodyIndex :type Integer) (bFromSweep :type Boolean) (SweepResult :type Hit%20Result%20Structure%20%28by%20ref%29))
  (if (!= OtherActor (Variables|Actor|GetInstigator))
    (Math|Integer|IncrementInt (Variables|Default|GetHitCount)
      (:%20%20
        (Class|IDamageable|Damage(Message) OtherActor (Variables|Default|GetProjectileDamage) 0.0 self (Transformation|GetActorLocation))
        (if (>= (Variables|Default|GetHitCount) (Variables|Default|GetMaxAmountOfHitEnemies))
          (Actor|DestroyActor))))))

(event EventBeginPlay)

(event Collision|EventActorBeginOverlap
  (params (OtherActor :type Actor%20Object%20Reference)))

(fn ConstructionScript
  (bind _projectilemovement (Variables|Default|GetProjectileMovement))
  (Actor|SetLifeSpan (Variables|Default|GetLifeSpan))
  (Variables|/Script/Engine.ProjectileMovementComponent|SetProjectileGravityScale _projectilemovement (Variables|Default|GetGravity))
  (Variables|/Script/Engine.ProjectileMovementComponent|SetInitialSpeed _projectilemovement (Variables|Default|GetStartSpeed))
  (Variables|/Script/Engine.ProjectileMovementComponent|SetMaxSpeed _projectilemovement (Variables|Default|GetMaxSpeed))
  (Transformation|SetWorldScale3D (Variables|Default|GetProjectileMesh) (Variables|Default|GetmeshScale)))
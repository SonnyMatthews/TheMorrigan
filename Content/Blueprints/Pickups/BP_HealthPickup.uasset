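; BP_HealthPickup is a pickup actor that gives health to the player on overlap.
; On BeginPlay it raises itself by its sphere's radius.
; When a component tagged "Player" enters the sphere, it prints a debug string and sends HealthToAdd to the owning actor through the IAddHealthMessage call.
; The pickup destroys itself only if that call returns true, so it remains otherwise.
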(event OnComponentBeginOverlap(Sphere)
  (params (OverlappedComponent :type Primitive%20Component%20Object%20Reference) (OtherActor :type Actor%20Object%20Reference) (OtherComp :type Primitive%20Component%20Object%20Reference) (OtherBodyIndex :type Integer) (bFromSweep :type Boolean) (SweepResult :type Hit%20Result%20Structure%20%28by%20ref%29))
  (bind _returnvalue (Components|ComponentHasTag OtherComp "Player"))
  (if _returnvalue
    (Development|PrintString (Utilities|String|ToString(Boolean) _returnvalue))
    (bind _hasaddedhealth_ (Class|ICharacter|IAddHealth(Message) OtherActor (Variables|Default|GetHealthToAdd)))
    (if _hasaddedhealth_
      (Actor|DestroyActor))))

(event EventBeginPlay
  (bind _returnvalue (Transformation|GetActorLocation))
  (Transformation|SetActorLocation (Math|Vector|MakeVector (.x _returnvalue) (.y _returnvalue) (+ (.z _returnvalue) (Variables|/Script/Engine.SphereComponent|GetSphereRadius (Variables|Default|GetSphere)))) false false))

(event EventTick
  (params (DeltaSeconds :type Float%20%28single-precision%29)))

(fn ConstructionScript)
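; BP_PickupUpgrade is an upgrade pickup that offers the player a choice of three room buff options.
; ITrigger arms it by attaching a particle emitter and enabling box collision, while IReset removes both on the game mode's Init Player Respawn state.
; A BP_BaseCharacter overlap pauses the game, opens the Widget_RoomBuff screen with those options, then destroys the pickup after a short delay.
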(event OnComponentBeginOverlap(Box)
  (params (OverlappedComponent :type Primitive%20Component%20Object%20Reference) (OtherActor :type Actor%20Object%20Reference) (OtherComp :type Primitive%20Component%20Object%20Reference) (OtherBodyIndex :type Integer) (bFromSweep :type Boolean) (SweepResult :type Hit%20Result%20Structure%20%28by%20ref%29))
  (if (Utilities|ClassIsChildOf (Utilities|GetClass OtherActor) "/Game/Blueprints/Pawn/BP_BaseCharacter.BP_BaseCharacter_C")
    (Game|SetGamePaused true)
    (bind _returnvalue (UserInterface|CreateWidget "/Game/Blueprints/UI/Widget_RoomBuff.Widget_RoomBuff_C" 0 (Variables|Default|GetOption%201) (Variables|Default|GetOption%202) (Variables|Default|GetOption%203)))
    (UserInterface|Viewport|AddtoViewport _returnvalue 0)
    (Utilities|FlowControl|Delay 0.1)
    (Actor|DestroyActor)))

(event Custom|OnNewGameState
  (params (NewState :type E_GameStates%20Enum :default "NewEnumerator0"))
  (switch Utilities|FlowControl|Switch|SwitchonE_GameStates NewState
    (:NewEnumerator10
      (CallFunction|IReset))))

(event Custom|OnBindToGameMode
  (bind _gamemode (Class|IMorriganGameMode|GetGameModeRef(Message) (Game|GetGameMode)))
  (EventDispatchers|BindEventtoOnNewState _gamemode (delegate Custom|OnNewGameState)))

(event EventBeginPlay
  (CallFunction|OnBindtoGameMode))

(event EventITrigger
  (bind _returnvalue (Effects|SpawnEmitterAttached (Variables|Default|GetParticle%20Effect) (Variables|Default|GetBox) "None" "0, 0, 0" "0, 0, 0" "0.150000,0.150000,0.150000"))
  (Variables|Default|SetEmitter _returnvalue)
  (Collision|SetCollisionEnabled (Variables|Default|GetBox) "QueryAndPhysics"))

(event EventIReset
  (bind _emitter (Variables|Default|GetEmitter))
  (Utilities|IsValid _emitter
    (:Is%20Valid
      (Components|DestroyComponent _emitter))
    (:Is%20Not%20Valid
      _))
  (Collision|SetCollisionEnabled (Variables|Default|GetBox) "NoCollision"))

(fn ConstructionScript)
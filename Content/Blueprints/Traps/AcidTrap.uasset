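; Acid trap that deals repeated toxic damage to actors inside its box, using stats read from a data table.
; Overlap events maintain a hit list; the first entry starts particles, steam sound and a looping timer that sends poison data to each listed actor through a damage message.
; When the list empties, the timer pauses, effects stop and the DoOnce gate resets.
; Init and Uninit events switch the trap on and off.
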(event OnComponentBeginOverlap(Box)
  (params (OverlappedComponent :type Primitive%20Component%20Object%20Reference) (OtherActor :type Actor%20Object%20Reference) (OtherComp :type Primitive%20Component%20Object%20Reference) (OtherBodyIndex :type Integer) (bFromSweep :type Boolean) (SweepResult :type Hit%20Result%20Structure%20%28by%20ref%29))
  ;[1 1 1] If actor hits collision, add to list, start the acid timer
  (Utilities|Array|AddUnique (Variables|Default|GetHitActors) OtherActor)
  (Utilities|FlowControl|DoOnce false
    (:Completed
      (Utilities|Time|UnpauseTimerbyHandle (Variables|Default|GetTimerHandle))
      (Components|Activation|Activate (Variables|Default|GetAcidParticles) false)
      (bind _returnvalue (Audio|SpawnSoundatLocation "/Game/StarterContent/Audio/Steam01_Cue.Steam01_Cue" (Transformation|GetActorLocation self) "0, 0, 0" 2.0 1.0 0.0 0 0))
      (bind _returnvalue_2 (Utilities|Time|SetTimerbyEvent (delegate Custom|AcidTickDamage) 0.5 true))
      (Variables|Default|SetTimerHandle _returnvalue_2))))

(event OnComponentEndOverlap(Box)
  (params (OverlappedComponent :type Primitive%20Component%20Object%20Reference) (OtherActor :type Actor%20Object%20Reference) (OtherComp :type Primitive%20Component%20Object%20Reference) (OtherBodyIndex :type Integer))
  (bind _hitactors (Variables|Default|GetHitActors))
  ;[1 1 1] If actor leaves, check if empty, if so pause acid tick and disable sound/particles
  (Utilities|Array|RemoveItem _hitactors OtherActor)
  (if (not (Utilities|Array|IsValidIndex _hitactors))
    (Utilities|Time|PauseTimerbyHandle (Variables|Default|GetTimerHandle))
    (Components|Activation|Deactivate (Variables|Default|GetAcidParticles))
    (Utilities|IsValid (stale OnComponentBeginOverlap(Box) _returnvalue)
      (:Is%20Valid
        (Audio|Components|Audio|Stop (stale OnComponentBeginOverlap(Box) _returnvalue))
        ;[1 1 1] If actor hits collision, add to list, start the acid timer
        (Utilities|FlowControl|DoOnce false) ; enters at Reset
      )
      (:Is%20Not%20Valid
        (Utilities|FlowControl|DoOnce false) ; enters at Reset
      ))))

(event Custom|AcidTickDamage
  ;[1 1 1] Acid tick damage function
  (for _array_element (Variables|Default|GetHitActors)
    (Class|IDamageable|ApplyToxicDamage(Message) _array_element self "0, 0, 0" (Variables|Default|GetPoisonData))))

(event EventInit
  ;[1 1 1] Init and uninit trap
  (Variables|/Script/Engine.PrimitiveComponent|SetbGenerateOverlapEvents (Variables|Default|GetBox) true)
  (bind _returnvalue (Utilities|GetDataTableRow (Variables|Default|GetStats) (Variables|Default|GetStatsRowName))
    (:then
      (Variables|Default|SetPoisonData (.AcidTrapData (Utilities|Struct|BreakS_TrapStats _returnvalue))))))

(event EventUninit
  ;[1 1 1] Init and uninit trap
  (Variables|/Script/Engine.PrimitiveComponent|SetbGenerateOverlapEvents (Variables|Default|GetBox) false)
  (Utilities|Time|ClearandInvalidateTimerbyHandle (Variables|Default|GetTimerHandle)))

(event EventBeginPlay
  ;[1 1 1] Init and uninit trap
  (Variables|/Script/Engine.PrimitiveComponent|SetbGenerateOverlapEvents (Variables|Default|GetBox) true)
  (bind _returnvalue (Utilities|GetDataTableRow (Variables|Default|GetStats) (Variables|Default|GetStatsRowName))
    (:then
      (Variables|Default|SetPoisonData (.AcidTrapData (Utilities|Struct|BreakS_TrapStats _returnvalue))))))

(fn ConstructionScript)
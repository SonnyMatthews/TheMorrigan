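; Trap pressure sensor that fires every linked arrow wall trap when something overlaps it.
; A held-down flag fires the traps once per activation and resets only when no actors remain on the collision.
; Init and BeginPlay enable overlaps and read arrow damage and lifetime from a stats data table.
; Uninit disables overlaps and clears the flag.
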(event OnComponentBeginOverlap(SensorCollision)
  (params (OverlappedComponent :type Primitive%20Component%20Object%20Reference) (OtherActor :type Actor%20Object%20Reference) (OtherComp :type Primitive%20Component%20Object%20Reference) (OtherBodyIndex :type Integer) (bFromSweep :type Boolean) (SweepResult :type Hit%20Result%20Structure%20%28by%20ref%29))
  ;[1 1 1] Sensor will shoot arrows out of all linked arrow wall traps once when activated, it will have to be stepped off again before it can be reactivated
  (if (not (Variables|Default|GetHeldDown))
    (Variables|Default|SetHeldDown true)
    (for _array_element (Variables|Default|GetArrowTrapRefs)
      (Default|ShootArrows _array_element))))

(event OnComponentEndOverlap(SensorCollision)
  (params (OverlappedComponent :type Primitive%20Component%20Object%20Reference) (OtherActor :type Actor%20Object%20Reference) (OtherComp :type Primitive%20Component%20Object%20Reference) (OtherBodyIndex :type Integer))
  ;[1 1 1] Sensor will shoot arrows out of all linked arrow wall traps once when activated, it will have to be stepped off again before it can be reactivated
  (if (not (Utilities|Array|IsValidIndex (Collision|GetOverlappingActors (Variables|Default|GetSensorCollision) 0 :!class /Script/Engine.PrimitiveComponent)))
    (Variables|Default|SetHeldDown false)))

(event EventBeginPlay
  ;[1 1 1] Init and uninit
  (Variables|/Script/Engine.PrimitiveComponent|SetbGenerateOverlapEvents (Variables|Default|GetSensorCollision) true)
  (bind _returnvalue (Utilities|GetDataTableRow (Variables|Default|GetStats) (Variables|Default|GetStatsRowName))
    (:then
      (Variables|Default|SetArrowDamage (.ArrowDamagePerHit (Utilities|Struct|BreakS_TrapStats _returnvalue)))
      (Variables|Default|SetArrowLifeTime (.ArrowLifeTime (Utilities|Struct|BreakS_TrapStats _returnvalue))))))

(event EventInit
  ;[1 1 1] Init and uninit
  (Variables|/Script/Engine.PrimitiveComponent|SetbGenerateOverlapEvents (Variables|Default|GetSensorCollision) true)
  (bind _returnvalue (Utilities|GetDataTableRow (Variables|Default|GetStats) (Variables|Default|GetStatsRowName))
    (:then
      (Variables|Default|SetArrowDamage (.ArrowDamagePerHit (Utilities|Struct|BreakS_TrapStats _returnvalue)))
      (Variables|Default|SetArrowLifeTime (.ArrowLifeTime (Utilities|Struct|BreakS_TrapStats _returnvalue))))))

(event EventUninit
  ;[1 1 1] Init and uninit
  (Variables|/Script/Engine.PrimitiveComponent|SetbGenerateOverlapEvents (Variables|Default|GetSensorCollision) false)
  (Variables|Default|SetHeldDown false))

(fn ConstructionScript)
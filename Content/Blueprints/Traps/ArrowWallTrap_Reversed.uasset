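; Wall arrow trap that fires repeated volleys while triggered by an actor overlap, damaging players in its arrow path.
; Overlap begin enables the arrow collision's overlap events, fires at once and starts a looping timer; overlap end disables them and clears the timer.
; Each volley restarts the particle effect, plays a sound and sends a damage message to every player character overlapping the arrow collision.
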(event Custom|ShootArrows
  (Components|Activation|Deactivate (Variables|Default|GetParticleSystem))
  (Components|Activation|Activate (Variables|Default|GetParticleSystem) false)
  (Audio|PlaySoundatLocation "/Game/SuperGrid/TutorialLevel/SoundEffects/PingBing.PingBing" (Transformation|GetActorLocation self) "0, 0, 0" 1.0 1.0 0.0 0 0 0)
  (for _array_element (Collision|GetOverlappingActors (Variables|Default|GetArrowCollision) "/Game/Blueprints/Pawn/BP_Char_Player.BP_Char_Player_C" :!class /Script/Engine.PrimitiveComponent)
    (Class|IDamageable|Damage(Message) _array_element (Variables|Default|GetArrowDamage) 0.0 self "0, 0, 0")))

(event Collision|EventActorEndOverlap
  (params (OtherActor :type Actor%20Object%20Reference))
  (Variables|/Script/Engine.PrimitiveComponent|SetbGenerateOverlapEvents (Variables|Default|GetArrowCollision) false)
  (Utilities|Time|ClearandInvalidateTimerbyHandle (Variables|Default|GetTimer)))

(event Collision|EventActorBeginOverlap
  (params (OtherActor :type Actor%20Object%20Reference))
  (Variables|/Script/Engine.PrimitiveComponent|SetbGenerateOverlapEvents (Variables|Default|GetArrowCollision) true)
  (CallFunction|ShootArrows)
  (bind _returnvalue (Utilities|Time|SetTimerbyEvent (delegate Custom|ShootArrows) (Variables|Default|GetTimeBetweenArrows) true))
  (Variables|Default|SetTimer _returnvalue))

(fn ConstructionScript)
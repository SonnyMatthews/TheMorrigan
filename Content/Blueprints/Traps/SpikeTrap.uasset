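; Spike trap actor that damages any actor overlapping it, immediately on entry and then at a repeating interval.
; Overlap begin adds the actor to a hit list, sends an interface damage message, plays particles and a chop sound, and sets a looping timer.
; ShootSpikes repeats the damage and effects for each listed actor.
; Overlap end removes the actor and clears the timer once the list is empty.
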(event Custom|ShootSpikes
  (bind _self self)
  (bind _particlesystem (Variables|Default|GetParticleSystem))
  (for _array_element (Variables|Default|GetActorsToHit)
    (Class|IDamageable|Damage(Message) _array_element (Variables|Default|GetDamage) 0.0 _self "0, 0, 0")
    (Components|Activation|Deactivate _particlesystem)
    (Components|Activation|Activate _particlesystem false)
    (Audio|PlaySoundatLocation "/Game/SuperGrid/TutorialLevel/SoundEffects/SimpleChop_A.SimpleChop_A" (Transformation|GetActorLocation _self) "0, 0, 0" 1.0 1.0 0.0 0 0 0)))

(event Collision|EventActorEndOverlap
  (params (OtherActor :type Actor%20Object%20Reference))
  (bind _actorstohit (Variables|Default|GetActorsToHit))
  (Utilities|Array|RemoveItem _actorstohit OtherActor)
  (if (not (Utilities|Array|IsValidIndex _actorstohit))
    (Utilities|Time|ClearandInvalidateTimerbyHandle (Variables|Default|GetHitTimer))))

(event Collision|EventActorBeginOverlap
  (params (OtherActor :type Actor%20Object%20Reference))
  (bind _self self)
  (Utilities|Array|AddUnique (Variables|Default|GetActorsToHit) OtherActor)
  (Class|IDamageable|Damage(Message) OtherActor (Variables|Default|GetDamage) 0.0 _self "0, 0, 0")
  (Components|Activation|Activate (Variables|Default|GetParticleSystem) false)
  (Audio|PlaySoundatLocation "/Game/SuperGrid/TutorialLevel/SoundEffects/SimpleChop_A.SimpleChop_A" (Transformation|GetActorLocation _self) "0, 0, 0" 1.0 1.0 0.0 0 0 0)
  (bind _returnvalue (Utilities|Time|SetTimerbyEvent (delegate Custom|ShootSpikes) (Variables|Default|GetTimeBetweenAttacks) true))
  (Variables|Default|SetHitTimer _returnvalue))

(fn ConstructionScript)
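; Swinging axe trap that damages actors its box overlaps, with a particle burst and chop sound on each hit.
; BeginPlay and Init enable overlaps, read per-hit damage from a stats data table row, then play a timeline that lerps the actor's rotation.
; Overlaps turn off when the timeline finishes, while Uninit only stops the swing.
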(event OnComponentBeginOverlap(Box)
  (params (OverlappedComponent :type Primitive%20Component%20Object%20Reference) (OtherActor :type Actor%20Object%20Reference) (OtherComp :type Primitive%20Component%20Object%20Reference) (OtherBodyIndex :type Integer) (bFromSweep :type Boolean) (SweepResult :type Hit%20Result%20Structure%20%28by%20ref%29))
  (bind _particlesystem (Variables|Default|GetParticleSystem))
  ;[1 1 1] If overlapped, damage, if particle is already playing disable then play again and then play sound
  (Class|IDamageable|Damage(Message) OtherActor (Variables|Default|GetDamage) 0.0 0 "0, 0, 0")
  (Components|Activation|Deactivate _particlesystem)
  (Components|Activation|Activate _particlesystem false)
  (Audio|PlaySoundatLocation "/Game/SuperGrid/TutorialLevel/SoundEffects/SimpleChop_A.SimpleChop_A" (Transformation|GetActorLocation OtherActor) "0, 0, 0" 1.0 1.0 0.0 0 0 0))

(event EventInit
  ;[1 1 1] Start axe swing on init and enable collision, on unit stop axe and disable
  (Variables|/Script/Engine.PrimitiveComponent|SetbGenerateOverlapEvents (Variables|Default|GetBox) true)
  (bind _returnvalue (Utilities|GetDataTableRow (Variables|Default|GetStats) (Variables|Default|GetStatsRowName))
    (:then
      (Variables|Default|SetDamage (.AxeDamagePerHit (Utilities|Struct|BreakS_TrapStats _returnvalue)))
      (bind _newtrack_0 (Timeline|Swing PlayFromStart)
        (:Update
          (Transformation|SetActorRotation (Math|Rotator|Lerp(Rotator) (Variables|Default|GetLerp%20rotator%20A) (Variables|Default|GetLerp%20rotator%20B) _newtrack_0)))
        (:Finished
          (Variables|/Script/Engine.PrimitiveComponent|SetbGenerateOverlapEvents (Variables|Default|GetBox) false))))))

(event EventBeginPlay
  ;[1 1 1] Start axe swing on init and enable collision, on unit stop axe and disable
  (Variables|/Script/Engine.PrimitiveComponent|SetbGenerateOverlapEvents (Variables|Default|GetBox) true)
  (bind _returnvalue (Utilities|GetDataTableRow (Variables|Default|GetStats) (Variables|Default|GetStatsRowName))
    (:then
      (Variables|Default|SetDamage (.AxeDamagePerHit (Utilities|Struct|BreakS_TrapStats _returnvalue)))
      (bind _newtrack_0 (Timeline|Swing PlayFromStart)
        (:Update
          (Transformation|SetActorRotation (Math|Rotator|Lerp(Rotator) (Variables|Default|GetLerp%20rotator%20A) (Variables|Default|GetLerp%20rotator%20B) _newtrack_0)))
        (:Finished
          (Variables|/Script/Engine.PrimitiveComponent|SetbGenerateOverlapEvents (Variables|Default|GetBox) false))))))

(event EventUninit
  ;[1 1 1] Start axe swing on init and enable collision, on unit stop axe and disable
  (bind _newtrack_0 (Timeline|Swing Stop)
    (:Update
      (Transformation|SetActorRotation (Math|Rotator|Lerp(Rotator) (Variables|Default|GetLerp%20rotator%20A) (Variables|Default|GetLerp%20rotator%20B) _newtrack_0)))
    (:Finished
      (Variables|/Script/Engine.PrimitiveComponent|SetbGenerateOverlapEvents (Variables|Default|GetBox) false))))

(fn ConstructionScript)
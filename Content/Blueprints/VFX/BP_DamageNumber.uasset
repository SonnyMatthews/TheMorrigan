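; BP_DamageNumber is a floating damage popup actor that shows rounded-up damage in a coloured W_damageNumber widget.
; On BeginPlay, damage relative to character max health sets a clamped scale, which drives randomised size, drift speed, slowdown and lifetime.
; Tick interpolates it up from zero while drifting and decelerating, then, after the lifetime timer, shrinks it at a jittered rate and destroys it.
; The MaxSize vector clamp in ApplyScale is disconnected and never runs.
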(event Custom|OnDie
  (Variables|Default|SetScaleDownRate (+ (Variables|Default|GetScaleDownRate) (Math|Random|RandomFloatinRange -2.5 2.5)))
  (Variables|Default|SetisAlive false))

(event EventBeginPlay
  (Transformation|SetActorScale3D "0, 0, 0")
  (bind _returnvalue (UserInterface|CreateWidget "/Game/Blueprints/Widgets/W_damageNumber.W_damageNumber_C"))
  (bind _output_get (Variables|Default|SetdamageVFXWidget _returnvalue))
  (UserInterface|SetWidget (Variables|Default|GetDamageWidget) _output_get)
  (Default|SetTextNumber (Variables|Default|GetdamageVFXWidget) (Math|Float|Ceil (Variables|Default|Getdamage)))
  (Default|SetTextColour (Variables|Default|GetdamageVFXWidget) (Variables|Default|GettextColour))
  (CallFunction|CalculateScale)
  (CallFunction|ApplyScale)
  (Variables|Default|SetisAlive true)
  (Utilities|Time|SetTimerbyEvent (delegate Custom|OnDie) (Variables|Default|GetlifeTime))
  (Variables|Default|SetIsInit true))

(event EventTick
  (params (DeltaSeconds :type Float%20%28single-precision%29))
  (if (Variables|Default|GetIsInit)
    (if (Variables|Default|GetisAlive)
      (Transformation|SetActorLocation (+ (Transformation|GetActorLocation) (* (* (Variables|Default|GetdriftDir) (Variables|Default|GetdriftSpeed)) DeltaSeconds)) false false)
      (Transformation|SetActorScale3D (Math|Interpolation|VInterpTo (Transformation|GetActorScale3D) (Variables|Default|GetmaxSize) DeltaSeconds (Variables|Default|GetScaleUpSpeed)))
      (Variables|Default|SetdriftSpeed (Math|Interpolation|FInterpTo (Variables|Default|GetdriftSpeed) 0.0 DeltaSeconds (Variables|Default|GetSlowDownRate)))
      (else
        (Transformation|SetActorScale3D (Math|Interpolation|VInterpTo (Transformation|GetActorScale3D) "0, 0, 0" DeltaSeconds (Variables|Default|GetScaleDownRate)))
        (if (<= (Math|Vector|VectorLength (Transformation|GetActorScale3D)) 0.0)
          (Actor|DestroyActor))))))

(fn ConstructionScript)

(fn CalculateScale
  (bind _output_get (LocalVariables|SetpercentChange (/ (Variables|Default|Getdamage) (Variables|Default|GetcharacterMaxHealth))))
  (Variables|Default|Setscale (Math|Float|Clamp(Float) (* _output_get (Variables|Default|GetscaleMultiplier)) 0.0 (Variables|Default|GetmaxScale))))

(fn ApplyScale
  (bind _returnvalue (Math|Random|RandomFloatinRange -0.1 0.1))
  (bind _scale (Variables|Default|Getscale))
  (bind _returnvalue_2 (+ _scale _returnvalue))
  (bind _output_get (Variables|Default|SetmaxSize (Math|Vector|MakeVector _returnvalue_2 _returnvalue_2 _returnvalue_2)))
  (Variables|Default|SetdriftSpeed (* (Variables|Default|GetdriftSpeed) (Variables|Default|Getscale)))
  (if (> (Variables|Default|Getscale) 1.0)
    (Variables|Default|SetSlowDownRate (+ (* (Variables|Default|GetSlowDownRate) (/ 1.0 (Variables|Default|Getscale))) (Math|Random|RandomFloatinRange -1.0 1.0)))
    (else
      (Variables|Default|SetSlowDownRate (+ (* (Variables|Default|Getscale) (Variables|Default|GetSlowDownRate)) (Math|Random|RandomFloatinRange -1.0 1.0)))))
  (Variables|Default|SetlifeTime (* (Variables|Default|GetlifeTime) (Variables|Default|Getscale))))
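; Floating text actor that shows a coloured damage-type or status label through a W_damageNumber widget.
; On BeginPlay it starts at zero scale, creates the widget, sets its text and colour, rolls a slightly randomised scale and calls ApplyScale.
; A lifetime timer then clears IsAlive and jitters the scale-down rate; the code that consumes these values is outside this file.
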(event Custom|CustomEvent
  (Variables|Default|SetScaleDownRate (+ (Variables|Default|GetScaleDownRate) (Math|Random|RandomFloatinRange -2.5 2.5)))
  (Variables|Default|SetisAlive false))

(event EventBeginPlay
  (Transformation|SetActorScale3D "0, 0, 0")
  (bind _returnvalue (UserInterface|CreateWidget "/Game/Blueprints/Widgets/W_damageNumber.W_damageNumber_C"))
  (bind _output_get (Variables|Default|SetdamageVFXWidget _returnvalue))
  (UserInterface|SetWidget (Variables|Default|GetDamageWidget) _output_get)
  (Default|SetWidgetText (Variables|Default|GetdamageVFXWidget) (Utilities|Text|ToText(String) (Variables|Default|GetstatusText)))
  (Default|SetTextColour (Variables|Default|GetdamageVFXWidget) (Variables|Default|GettextColour))
  (CallFunction|CalculateScale)
  (CallFunction|ApplyScale)
  (Variables|Default|SetisAlive true)
  (Utilities|Time|SetTimerbyEvent (delegate Custom|CustomEvent) (Variables|Default|GetlifeTime))
  (Variables|Default|SetIsInit true))

(fn ConstructionScript
  (|CallParentFunction))

(fn CalculateScale
  (Variables|Default|Setscale (Math|Random|RandomFloatinRange 0.8 1.2)))
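; BP_EnemySpawnCircle is a VFX actor that, judging by its name, marks an enemy spawn with a growing, spinning circle.
; On BeginPlay, timelines scale the root up from zero and accelerate its yaw spin, which Tick applies every frame.
; Calling Dissapear reverses the spin, shrinks the root to zero and destroys the actor.
; Timeline updates lerp from the current value rather than a stored start, so easing compounds each update.
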(event Custom|AccelerateRotation
  (bind _acceleration (Timeline|RotAccelTime PlayFromStart)
    (:Update
      (Variables|Default|SetcurrentRotationspeed (Math|Float|Lerp (Variables|Default|GetcurrentRotationspeed) (Variables|Default|GetmaxRotSpeed) _acceleration)))))

(event Custom|ScaleDown
  (bind _scaledown (Timeline|ScaleDownTime PlayFromStart)
    (:Update
      (Transformation|SetWorldScale3D (Variables|Default|GetDefaultSceneRoot) (Math|Vector|Lerp(Vector) (Transformation|GetWorldScale (Variables|Default|GetDefaultSceneRoot)) "0, 0, 0" _scaledown)))
    (:Finished
      (Actor|DestroyActor))))

(event Custom|Dissapear
  (Variables|Default|SetisDone true)
  (Components|Timeline|SetPlayRate (Variables|Default|GetScaleDownTime) 1.5)
  (CallFunction|ScaleDown))

(event Custom|ScaleUp
  (bind _acceleration (Timeline|ScaleUpTime PlayFromStart)
    (:Update
      (Transformation|SetWorldScale3D (Variables|Default|GetDefaultSceneRoot) (Math|Vector|Lerp(Vector) (Transformation|GetWorldScale (Variables|Default|GetDefaultSceneRoot)) (Variables|Default|GetmaxScale) _acceleration)))))

(event EventBeginPlay
  (Transformation|SetWorldScale3D (Variables|Default|GetDefaultSceneRoot) "0, 0,0.000000")
  (Components|Timeline|SetPlayRate (Variables|Default|GetScaleUpTime) 0.3)
  (Components|Timeline|SetPlayRate (Variables|Default|GetRotAccelTime) 0.6)
  (CallFunction|ScaleUp)
  (CallFunction|AccelerateRotation))

(event EventTick
  (params (DeltaSeconds :type Float%20%28single-precision%29))
  (if (Variables|Default|GetisDone)
    (Transformation|SetWorldRotation (Variables|Default|GetDefaultSceneRoot) (Math|Rotator|MakeRotator 0.0 0.0 (- (.yaw (Transformation|GetWorldRotation (Variables|Default|GetDefaultSceneRoot))) (* DeltaSeconds (Variables|Default|GetcurrentRotationspeed)))) false false)
    (else
      (Transformation|SetWorldRotation (Variables|Default|GetDefaultSceneRoot) (Math|Rotator|MakeRotator 0.0 0.0 (+ (.yaw (Transformation|GetWorldRotation (Variables|Default|GetDefaultSceneRoot))) (* DeltaSeconds (Variables|Default|GetcurrentRotationspeed)))) false false))))

(fn ConstructionScript)
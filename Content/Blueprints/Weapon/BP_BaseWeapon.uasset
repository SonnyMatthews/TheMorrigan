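; Base weapon actor that deals damage and knockback for its parent actor through a toggled hitbox or an instant AOE sphere.
; Box overlaps hit each tagged actor once per activation, running DamageCalc, crit or life-steal popup text and an OnAttack call.
; AOE sends raw damage to BP_BaseEnemy pawns, skipping those steps.
; DamageCalc is a zero-damage stub, presumably for child overrides; helpers cover data-table stats and status-effect particles.
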(event OnComponentBeginOverlap(Box)
  (params (OverlappedComponent :type Primitive%20Component%20Object%20Reference) (OtherActor :type Actor%20Object%20Reference) (OtherComp :type Primitive%20Component%20Object%20Reference) (OtherBodyIndex :type Integer) (bFromSweep :type Boolean) (SweepResult :type Hit%20Result%20Structure%20%28by%20ref%29))
  ;[1 1 1] Overlap
  (if (not (Utilities|Array|ContainsItem (Variables|Default|GetHitActors) OtherActor))
    (if (Components|ComponentHasTag OtherComp (Variables|Default|GetActorToHitTag))
      (if (not (== (Actor|GetParentActor) OtherActor))
        (Utilities|Array|AddUnique (Variables|Default|GetHitActors) OtherActor)
        (bind (_damage _damagetype) (CallFunction|DamageCalc (Variables|Default|GetTempDamage)))
        (CallFunction|DamageTypeVFX _damagetype (Transformation|GetActorLocation OtherActor))
        (Default|CallOnAttack OtherActor)
        (Class|IDamageable|Damage(Message) OtherActor _damage (Variables|Default|GetTempKnockback) self (Transformation|GetActorLocation (Actor|GetParentActor)))))))

(event EventBeginPlay)

(event EventSetDamageMultiplier
  (params (Dmg%20Multiplier :type Float%20%28single-precision%29))
  (Variables|Default|SetDamage%20Multiplier Dmg%20Multiplier))

(event EventIActivateWeaponHitbox
  (params (Damage :type Float%20%28single-precision%29) (Knockback :type Float%20%28single-precision%29) (DamageType :type EDamageApplicationType%20Enum :default "NewEnumerator0") (HitBoxSize :type Vector :default "0, 0, 0") (AOE_Size :type Float%20%28single-precision%29))
  ;[1 1 1] Hit Box Activation
  (Variables|Default|SetTempAOE_Size AOE_Size)
  (Variables|Default|SetTempHitBoxSize HitBoxSize)
  (Variables|Default|SetTempDamage Damage)
  (Variables|Default|SetTempKnockback Knockback)
  (bind _output_get (Variables|Default|SetTempDamageType DamageType))
  (switch Utilities|FlowControl|Switch|SwitchonEDamageApplicationType _output_get
    (:NewEnumerator0
      (Components|Box|SetBoxExtent (Variables|Default|GetBox) (Variables|Default|GetTempHitBoxSize) true)
      (Rendering|SetVisibility (Variables|Default|GetBox) false false)
      (Collision|SetCollisionEnabled (Variables|Default|GetBox) "QueryOnly"))
    (:NewEnumerator1
      (bind _outactors (Collision|SphereOverlapActors (Transformation|GetWorldLocation (Variables|Default|GetAOE_Location)) (Variables|Default|GetTempAOE_Size) (Utilities|Array|MakeArray "ObjectTypeQuery3") "/Game/Blueprints/AI/Characters/BP_BaseEnemy.BP_BaseEnemy_C" (Utilities|Array|MakeArray (Actor|GetParentActor))))
      (for _array_element _outactors
        (Class|IDamageable|Damage(Message) _array_element (Variables|Default|GetTempDamage) (Variables|Default|GetTempKnockback) self (Transformation|GetActorLocation))))))

(event EventIDeactivateWeaponHitbox
  ;[1 1 1] Hit Box Activation
  (Rendering|SetVisibility (Variables|Default|GetBox) false false)
  (Collision|SetCollisionEnabled (Variables|Default|GetBox) "NoCollision")
  (Utilities|Array|Clear (Variables|Default|GetHitActors)))

(fn ConstructionScript)

(fn GetDamageinRange
  (bind _weapondata (Variables|Default|GetWeaponData))
  (return (Math|Random|RandomFloatinRange (.mindamage _weapondata) (.maxdamage _weapondata))))

(fn SetWeaponData
  (params (DataTable :type Data%20Table%20Object%20Reference) (RowName :type Name))
  (bind _returnvalue (Utilities|GetDataTableRow DataTable RowName)
    (:then
      (bind _structout (Utilities|Struct|SetmembersinS_MeleeWeaponData _returnvalue (* (.minDamage (Utilities|Struct|BreakS_MeleeWeaponData _returnvalue)) (Variables|Default|GetDamage%20Multiplier)) (* (.maxDamage (Utilities|Struct|BreakS_MeleeWeaponData _returnvalue)) (Variables|Default|GetDamage%20Multiplier))))
      (bind _output_get (Variables|Default|SetWeaponData _structout))
      (bind _structout_2 (Utilities|Struct|SetmembersinS_MeleeWeaponData _output_get))
      (Variables|Default|SetActorToHitTag (Utilities|String|StringToName (.actortohittag _structout_2))))))

(fn GetKnockbackinRange
  (bind _weapondata (Variables|Default|GetWeaponData))
  (return (Math|Random|RandomFloatinRange (.maxknockback _weapondata) (.minknockback _weapondata))))

(fn DamageCalc
  (params (TempDamage :type Float%20%28single-precision%29))
  (return 0.0 "NewEnumerator2"))

(fn DamageTypeVFX
  (params (type :type E_DamageType%20Enum :default "NewEnumerator0") (otherActorLocation :type Vector))
  (bind (_x _y _z) (Math|Vector|BreakVector otherActorLocation))
  (bind _point (Class|IPawn|IRandomPointinSphere(Message) (Actor|GetParentActor) (Math|Vector|MakeVector _x _y (+ _z 1e+02)) 1e+01))
  (LocalVariables|SetspawnPoint _point)
  (LocalVariables|Setdir (Math|Vector|GetUnitDirection(Vector) (Transformation|GetActorLocation (Actor|GetParentActor)) otherActorLocation))
  (switch Utilities|FlowControl|Switch|SwitchonE_DamageType type
    (:NewEnumerator0
      (Game|SpawnActorfromClass "/Game/Blueprints/VFX/BP_DamageTypeText.BP_DamageTypeText_C" (Math|Transform|MakeTransform (LocalVariables|GetspawnPoint) "0, 0, 0" "1,1,1") "Undefined" 0 "CRIT" 0.0 "(R=1.000000,G=0.221798,B=0.021320,A=1.000000)" (LocalVariables|Getdir) 0.0 0))
    (:NewEnumerator1
      (Game|SpawnActorfromClass "/Game/Blueprints/VFX/BP_DamageTypeText.BP_DamageTypeText_C" (Math|Transform|MakeTransform (LocalVariables|GetspawnPoint) "0, 0, 0" "1,1,1") "Undefined" 0 "++" 0.0 "(R=0.000000,G=1.000000,B=0.246004,A=1.000000)" (LocalVariables|Getdir) 0.0 0))))

(fn EnableStatusEffectVFX
  (params (statusEffect :type E_StatusEffect%20Enum :default "NewEnumerator0"))
  (switch Utilities|FlowControl|Switch|SwitchonE_StatusEffect statusEffect
    (:NewEnumerator0
      (Effects|SpawnEmitterAttached "/Game/InfinityBladeEffects/Effects/FX_Skill_Aura/P_AuraCircle_Default_Base_01.P_AuraCircle_Default_Base_01" (Variables|Default|GetPaticleEffects) "None" "0, 0, 0" "0, 0, 0" "1.000000,1.000000,1.000000" "KeepRelativeOffset" false))
    (:NewEnumerator1
      (Effects|SpawnEmitterAttached "/Game/ParticleSystem/P_PoisonMist.P_PoisonMist" (Variables|Default|GetPaticleEffects) "None" "0, 0, 0" "0, 0, 0" "1.000000,1.000000,1.000000" "KeepRelativeOffset" false))))
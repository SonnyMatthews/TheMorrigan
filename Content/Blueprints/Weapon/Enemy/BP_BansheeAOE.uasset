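; Banshee area-of-effect attack actor that damages and knocks back Player-tagged actors, ignoring its instigator.
; OnAttack plays a sound, spawns the attack particle effect and resizes the Collision sphere to AttackRadius with an overlap update.
; Begin-overlap events on that sphere send DamageMessage to each hit player, crediting the instigator.
; The actor destroys itself when the particle system finishes.
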(event OnComponentBeginOverlap(Collision)
  (params (OverlappedComponent :type Primitive%20Component%20Object%20Reference) (OtherActor :type Actor%20Object%20Reference) (OtherComp :type Primitive%20Component%20Object%20Reference) (OtherBodyIndex :type Integer) (bFromSweep :type Boolean) (SweepResult :type Hit%20Result%20Structure%20%28by%20ref%29))
  (bind _instigator (Variables|Actor|GetInstigator))
  (if (!= OtherActor _instigator)
    (if (Actor|ActorHasTag OtherActor "Player")
      (Class|IDamageable|Damage(Message) OtherActor (Variables|Default|GetDamage) (Variables|Default|GetKnocBack) _instigator))))

(event Custom|OnAttack
  (Audio|SpawnSoundatLocation "/Game/MedievalCombatSounds/Magic/wav/Evil_Attack_01.Evil_Attack_01" (Transformation|GetActorLocation) "0, 0, 0" 1.0 1.0 0.0 0 0)
  (Components|Activation|SetActive (Variables|Default|GetCollision) false false)
  (Components|Sphere|SetSphereRadius (Variables|Default|GetCollision) (Variables|Default|GetAttackRadius) true)
  (bind _returnvalue (Effects|SpawnEmitteratLocation (Variables|Default|GetAttackVFX) (Transformation|GetActorLocation) "0, 0, 0" (Transformation|GetActorScale3D)))
  (EventDispatchers|BindEventtoOnSystemFinished _returnvalue (delegate Custom|AttackFinished)))

(event Custom|AttackFinished
  (params (PSystem :type Particle%20System%20Component%20Object%20Reference))
  (Components|DestroyComponent PSystem)
  (Actor|DestroyActor))

(event EventBeginPlay
  (Components|Activation|SetActive (Variables|Default|GetCollision) false false))

(fn ConstructionScript)
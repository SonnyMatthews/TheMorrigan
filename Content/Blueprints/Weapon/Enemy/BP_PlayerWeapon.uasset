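; Player weapon Blueprint that adjusts outgoing damage and its damage type according to the active boon reported by the Game Instance.
; DamageCalc sends the crit boon to a random crit roll that multiplies damage, and the life steal boon to a heal on the parent actor for a small percentage of damage.
; Life steal is skipped when the hit actor's shield is active, and the speed boon leaves damage unchanged.
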(event EventBeginPlay)

(event Collision|EventActorBeginOverlap
  (params (OtherActor :type Actor%20Object%20Reference)))

(event EventTick
  (params (DeltaSeconds :type Float%20%28single-precision%29)))

(fn ConstructionScript
  (|CallParentFunction))

(fn DamageCalc
  (params (TempDamage :type Float%20%28single-precision%29) (ActorHit :type Actor%20Object%20Reference))
  (bind _boon (Class|IInstance|GetActiveBoon(Message) (Game|GetGameInstance)))
  (switch Utilities|FlowControl|Switch|SwitchonEnum_Boons _boon
    (:NewEnumerator0
      (bind (_newdamage _damagetype) (CallFunction|CritDamage TempDamage))
      (return _newdamage _damagetype))
    (:NewEnumerator1
      (bind _isactive (Class|IElite|IsShieldActive(Message) ActorHit))
      (if _isactive
        _
        (else
          (bind _newdamage_2 (CallFunction|LifeSteal TempDamage))
          (return _newdamage_2 "NewEnumerator1"))))
    (:NewEnumerator2
      _))
  (return TempDamage "NewEnumerator2"))

(fn LifeSteal
  (params (Damage :type Float%20%28single-precision%29))
  (Class|ICharacter|IAddHealth(Message) (Actor|GetParentActor) (* (/ Damage 1e+02) 5.0))
  (return Damage))

(fn CritDamage
  (params (Damage :type Float%20%28single-precision%29))
  (if (> (Variables|Default|GetCritChance) (Math|Random|RandomFloatinRange 0.0 1.0))
    (return (* Damage (Variables|Default|GetCritMultiplier)) "NewEnumerator0")
    (else
      (return Damage "NewEnumerator2"))))
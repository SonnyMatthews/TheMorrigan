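; Enemy poison spell projectile that damages player components its sphere overlaps, ignoring its own instigator.
; Each hit sends direct damage and a timed toxic damage-over-time effect with a random-range tick amount through message calls on the hit actor.
; Hits are counted, and at the maximum KillProjectile spawns a poison explosion emitter at its location and destroys the actor.
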(event OnComponentBeginOverlap(Sphere)
  (params (OverlappedComponent :type Primitive%20Component%20Object%20Reference) (OtherActor :type Actor%20Object%20Reference) (OtherComp :type Primitive%20Component%20Object%20Reference) (OtherBodyIndex :type Integer) (bFromSweep :type Boolean) (SweepResult :type Hit%20Result%20Structure%20%28by%20ref%29))
  (bind _instigator (Variables|Default|GetInstigator))
  (if (and (!= OtherActor _instigator) (Components|ComponentHasTag OtherComp "Player"))
    (Math|Integer|IncrementInt (Variables|Default|GetHitCount)
      (:%20%20
        (Class|IDamageable|Damage(Message) OtherActor (Variables|Default|GetProjectileDamage) 0.0 _instigator (Transformation|GetActorLocation))
        (Class|IDamageable|ApplyToxicDamage(Message) OtherActor 0 "0, 0, 0" (Utilities|Struct|MakeS_ToxinData 5.0 1.25 1e+01 2e+01))
        (if (>= (Variables|Default|GetHitCount) (Variables|Default|GetMaxAmountOfHitEnemies))
          (CallFunction|KillProjectile))))))

(event EventBeginPlay
  (|CallParentFunction) ; This node is disabled and will not be called.\nDrag off pins to build functionality.
)

(event EventTick
  (params (DeltaSeconds :type Float%20%28single-precision%29))
  (|CallParentFunction DeltaSeconds) ; This node is disabled and will not be called.\nDrag off pins to build functionality.
)

(fn ConstructionScript
  (|CallParentFunction))

(fn KillProjectile
  (bind _returnvalue (Transformation|GetActorLocation))
  (Effects|SpawnEmitteratLocation "/Game/ParticleSystem/P_PoisonExplosion.P_PoisonExplosion" (Math|Vector|MakeVector (.x _returnvalue) (.y _returnvalue) (.z _returnvalue)))
  (Actor|DestroyActor))
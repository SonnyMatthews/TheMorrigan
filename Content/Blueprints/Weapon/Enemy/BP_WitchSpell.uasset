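; BP_WitchSpell is an enemy weapon projectile for the witch's spell that damages actors it overlaps.
; Its Sphere overlap ignores the instigator, counts each hit and sends a DamageMessage with zero knockback, crediting the instigator.
; It destroys itself once the hit count reaches MaxAmountOfHitEnemies, so it can pass through targets until that limit.
; BeginPlay and construction defer to the parent class.
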(event OnComponentBeginOverlap(Sphere)
  (params (OverlappedComponent :type Primitive%20Component%20Object%20Reference) (OtherActor :type Actor%20Object%20Reference) (OtherComp :type Primitive%20Component%20Object%20Reference) (OtherBodyIndex :type Integer) (bFromSweep :type Boolean) (SweepResult :type Hit%20Result%20Structure%20%28by%20ref%29))
  (bind _instigator (Variables|Default|GetInstigator))
  (if (!= OtherActor _instigator)
    (Math|Integer|IncrementInt (Variables|Default|GetHitCount)
      (:%20%20
        (Class|IDamageable|Damage(Message) OtherActor (Variables|Default|GetProjectileDamage) 0.0 _instigator)
        (if (>= (Variables|Default|GetHitCount) (Variables|Default|GetMaxAmountOfHitEnemies))
          (Actor|DestroyActor))))))

(event EventBeginPlay
  (|CallParentFunction))

(event Collision|EventActorBeginOverlap
  (params (OtherActor :type Actor%20Object%20Reference)))

(event EventTick
  (params (DeltaSeconds :type Float%20%28single-precision%29)))

(fn ConstructionScript
  (|CallParentFunction))